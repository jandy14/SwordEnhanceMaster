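; House main screen actor whose touch buttons lead to the main menu, guild, enhancement and laboratory, plus a dungeon button that opens a one-button message window.
; Each button fires only when touch release matches the component stored in EnableButton on press.
; Main and guild buttons call the scene manager; enhancement and lab timelines slide ActorHouseMenu in opposite X directions.
; Collision gates input: off at BeginPlay and during slides, then enabled on the destination panel.
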(event `self.ReceiveBeginPlay`
  ;[1 1 1] 초기화
  (`self.SetActorEnableCollision` false))

(event `self.Dungeon_Button.OnInputTouchEnd`
  (params (FingerIndex :type "ETouchIndex Enum" :default "Touch1") (TouchedComponent :type "PrimitiveComponent Object Reference"))
  (if (== TouchedComponent (`self.enableButton`))
    (message `/Game/Blueprints/WindowManager.CallOneButtonWindow` (`self.actor_OneButtonWindow`) "진동이 사라졌다!" self)))

(event `self.Dungeon_Button.OnInputTouchBegin`
  (params (FingerIndex :type "ETouchIndex Enum" :default "Touch1") (TouchedComponent :type "PrimitiveComponent Object Reference"))
  (set `self.enableButton` TouchedComponent))

(event `self.BlankButton_Sprite.OnInputTouchEnd`
  (params (FingerIndex :type "ETouchIndex Enum" :default "Touch1") (TouchedComponent :type "PrimitiveComponent Object Reference"))
  ;[1 1 1] 메인 메뉴로 가기
  (if (== TouchedComponent (`self.enableButton`))
    (message `/Game/Blueprints/GameManager/GameManagerInterface.CallScene_Main` (`self.actor_SceneManager`))))

(event `self.BlankButton_Sprite.OnInputTouchBegin`
  (params (FingerIndex :type "ETouchIndex Enum" :default "Touch1") (TouchedComponent :type "PrimitiveComponent Object Reference"))
  ;[1 1 1] 메인 메뉴로 가기
  (set `self.enableButton` TouchedComponent))

(event `self.Button_ToGuild.OnInputTouchEnd`
  (params (FingerIndex :type "ETouchIndex Enum" :default "Touch1") (TouchedComponent :type "PrimitiveComponent Object Reference"))
  ;[1 1 1] 용사길드로 씬 전환
  (if (== TouchedComponent (`self.enableButton`))
    (message `/Game/Blueprints/GameManager/GameManagerInterface.CallScene_Guild` (`self.actor_SceneManager`))))

(event `self.Button_ToGuild.OnInputTouchBegin`
  (params (FingerIndex :type "ETouchIndex Enum" :default "Touch1") (TouchedComponent :type "PrimitiveComponent Object Reference"))
  ;[1 1 1] 용사길드로 씬 전환
  (set `self.enableButton` TouchedComponent))

(event `self.Button_ToEnhancement.OnInputTouchEnd`
  (params (FingerIndex :type "ETouchIndex Enum" :default "Touch1") (TouchedComponent :type "PrimitiveComponent Object Reference"))
  ;[1 1 1] 강화하러 가기
  (if (== TouchedComponent (`self.enableButton`))
    (`self.SetActorEnableCollision` false)
    (set `self.vector_OriginalLocation` (`self.K2_GetActorLocation` (`self.actor_HouseMenu`)))
    (bind (_direction `_인터페이스_이동`) (`Timeline|ToEnhancement` :!via `PlayFromStart`)
      (:`Update`
        (`self.K2_SetActorLocation` (`self.actor_HouseMenu`) (+ (`KismetMathLibrary.MakeVector` (* `_인터페이스_이동` -288.0)) (`self.vector_OriginalLocation`)) false false))
      (:`Finished`
        (`self.SetActorEnableCollision` (`self.actor_Enhancement`) true)
        (message `/Game/Blueprints/WindowManager.RefreshProgressBar` (`self.actor_ProgressBar`) 0.0)))))

(event `self.Button_ToEnhancement.OnInputTouchBegin`
  (params (FingerIndex :type "ETouchIndex Enum" :default "Touch1") (TouchedComponent :type "PrimitiveComponent Object Reference"))
  ;[1 1 1] 강화하러 가기
  (set `self.enableButton` TouchedComponent))

(event `self.Button_ToLab.OnInputTouchEnd`
  (params (FingerIndex :type "ETouchIndex Enum" :default "Touch1") (TouchedComponent :type "PrimitiveComponent Object Reference"))
  ;[1 1 1] 연구실로 이동
  (if (== TouchedComponent (`self.enableButton`))
    (`self.SetActorEnableCollision` false)
    (set `self.vector_OriginalLocation` (`self.K2_GetActorLocation` (`self.actor_HouseMenu`)))
    (bind (_direction `_인터페이스_이동`) (`Timeline|타임라인_1` :!via `PlayFromStart`)
      (:`Update`
        (`self.K2_SetActorLocation` (`self.actor_HouseMenu`) (+ (`KismetMathLibrary.MakeVector` (* `_인터페이스_이동` 288.0)) (`self.vector_OriginalLocation`)) false false))
      (:`Finished`
        (`self.SetActorEnableCollision` (`self.actor_Laboratory`) true)))))

(event `self.Button_ToLab.OnInputTouchBegin`
  (params (FingerIndex :type "ETouchIndex Enum" :default "Touch1") (TouchedComponent :type "PrimitiveComponent Object Reference"))
  ;[1 1 1] 연구실로 이동
  (set `self.enableButton` TouchedComponent))

(fn `UserConstructionScript`)