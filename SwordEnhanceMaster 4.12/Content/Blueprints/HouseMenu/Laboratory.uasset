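; Laboratory screen of the house menu, where touch buttons change lab and house levels, sell sword-unlock hints and slide the menu back.
; Upgrades check level caps and money, then save and refresh the info bar; hint and house costs are zero placeholders.
; OpenHint picks a random unlockable sword and decodes its packed condition from SwordList for a partly randomized hint message.
; House upgrade is unfinished: its locked-sword check always returns false, skipping its hint.
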(event OnInputTouchEnd(Button_HouseLevelUp)
  (params (FingerIndex :type ETouchIndex%20Enum :default "Touch1") (TouchedComponent :type Primitive%20Component%20Object%20Reference))
  ;[1 0 0] 연구_집레벨----------------- 나중에 해야함
  (if (== TouchedComponent (Variables|Default|GetenableButton))
    (if (< (Variables|/Game/Blueprints/GameSetting/GameSaveData.GameSaveData_C|GethouseLevel (Variables|/Game/Blueprints/GameManager/GameManager.GameManager_C|GetgameSaveDataObject (Variables|Default|Getactor_GameManager))) 5) ; 집연구가 최고 레벨전인지
      (if (>= (Variables|/Game/Blueprints/GameSetting/GameSaveData.GameSaveData_C|Getmoney (Variables|/Game/Blueprints/GameManager/GameManager.GameManager_C|GetgameSaveDataObject (Variables|Default|Getactor_GameManager))) 0.0) ; 돈이 충분한지
        (Variables|/Game/Blueprints/GameSetting/GameSaveData.GameSaveData_C|Setmoney (Variables|/Game/Blueprints/GameManager/GameManager.GameManager_C|GetgameSaveDataObject (Variables|Default|Getactor_GameManager)) (- (Variables|/Game/Blueprints/GameSetting/GameSaveData.GameSaveData_C|Getmoney (Variables|/Game/Blueprints/GameManager/GameManager.GameManager_C|GetgameSaveDataObject (Variables|Default|Getactor_GameManager))) 0.0))
        (Variables|/Game/Blueprints/GameSetting/GameSaveData.GameSaveData_C|SethouseLevel (Variables|/Game/Blueprints/GameManager/GameManager.GameManager_C|GetgameSaveDataObject (Variables|Default|Getactor_GameManager)) (+ (Variables|/Game/Blueprints/GameSetting/GameSaveData.GameSaveData_C|GethouseLevel (Variables|/Game/Blueprints/GameManager/GameManager.GameManager_C|GetgameSaveDataObject (Variables|Default|Getactor_GameManager))) 1))
        (if (< (Variables|/Game/Blueprints/GameSetting/GameSaveData.GameSaveData_C|GetlabLevel (Variables|/Game/Blueprints/GameManager/GameManager.GameManager_C|GetgameSaveDataObject (Variables|Default|Getactor_GameManager))) 10) ; 연구 최고 레벨인지
          (Variables|/Game/Blueprints/GameSetting/GameSaveData.GameSaveData_C|SetlabLevel (Variables|/Game/Blueprints/GameManager/GameManager.GameManager_C|GetgameSaveDataObject (Variables|Default|Getactor_GameManager)) (+ (Variables|/Game/Blueprints/GameSetting/GameSaveData.GameSaveData_C|GetlabLevel (Variables|/Game/Blueprints/GameManager/GameManager.GameManager_C|GetgameSaveDataObject (Variables|Default|Getactor_GameManager))) 1)))
        (bind _개방안된게_있는지 (|개방안된게있는지확인_2_2))
        (if _개방안된게_있는지 ; 개방이 안된게 있나
          (bind (_개방되는_검 _하위_검 _소재_강화 _예리함_강화 _무게감_강화 _속성_강화) (CallFunction|OpenHint))
          (if (Utilities|Enum|NotEqual(Enum) _속성_강화 (Utilities|Text|MakeLiteralText "null")) ; 명검인지 아닌지(속성유무로 판단)
            (Class|WindowManager|CallOneButtonWindow(Message) (Variables|Default|Getactor_OneButtonWindow) (Utilities|String|Append (Utilities|String|Append "연구 레벨" (Utilities|String|ToString(Integer) (Variables|/Game/Blueprints/GameSetting/GameSaveData.GameSaveData_C|GetlabLevel (Variables|/Game/Blueprints/GameManager/GameManager.GameManager_C|GetgameSaveDataObject (Variables|Default|Getactor_GameManager)))) "<br>집레벨" (Utilities|String|ToString(Integer) (Variables|/Game/Blueprints/GameSetting/GameSaveData.GameSaveData_C|GethouseLevel (Variables|/Game/Blueprints/GameManager/GameManager.GameManager_C|GetgameSaveDataObject (Variables|Default|Getactor_GameManager))))) "<br>" (|힌트말만듦(명검)_2_2 _하위_검 _소재_강화 _예리함_강화 _무게감_강화 _속성_강화)) self) ; 힌트가 명검일 경우
            (else
              (Class|WindowManager|CallOneButtonWindow(Message) (Variables|Default|Getactor_OneButtonWindow) (Utilities|String|Append (Utilities|String|Append "연구 레벨" (Utilities|String|ToString(Integer) (Variables|/Game/Blueprints/GameSetting/GameSaveData.GameSaveData_C|GetlabLevel (Variables|/Game/Blueprints/GameManager/GameManager.GameManager_C|GetgameSaveDataObject (Variables|Default|Getactor_GameManager)))) "<br>집레벨" (Utilities|String|ToString(Integer) (Variables|/Game/Blueprints/GameSetting/GameSaveData.GameSaveData_C|GethouseLevel (Variables|/Game/Blueprints/GameManager/GameManager.GameManager_C|GetgameSaveDataObject (Variables|Default|Getactor_GameManager))))) "<br>" (|힌트말만듦(일반)_2_2 _하위_검 _소재_강화 _예리함_강화 _무게감_강화 _속성_강화)) self) ; 힌트가 일반일 경우
            ))
          (else
            (Class|WindowManager|CallOneButtonWindow(Message) (Variables|Default|Getactor_OneButtonWindow) (Utilities|String|Append "연구 레벨" (Utilities|String|ToString(Integer) (Variables|/Game/Blueprints/GameSetting/GameSaveData.GameSaveData_C|GetlabLevel (Variables|/Game/Blueprints/GameManager/GameManager.GameManager_C|GetgameSaveDataObject (Variables|Default|Getactor_GameManager)))) "<br>집레벨" (Utilities|String|ToString(Integer) (Variables|/Game/Blueprints/GameSetting/GameSaveData.GameSaveData_C|GethouseLevel (Variables|/Game/Blueprints/GameManager/GameManager.GameManager_C|GetgameSaveDataObject (Variables|Default|Getactor_GameManager))))) self) ; 힌트없을경우
          ))
        (SaveGame|SaveGametoSlot (Variables|/Game/Blueprints/GameManager/GameManager.GameManager_C|GetgameSaveDataObject (Variables|Default|Getactor_GameManager)) "GameSaveSlot1")
        (Class|WindowManager|RefreshTextBar(Message) (Variables|Default|Getactor_UserInfoBar))
        (else
          (Class|WindowManager|CallOneButtonWindow(Message) (Variables|Default|Getactor_OneButtonWindow) "돈 부족" self)))
      (else
        (Class|WindowManager|CallOneButtonWindow(Message) (Variables|Default|Getactor_OneButtonWindow) "집이 최고 레벨" self)))))

(event OnInputTouchBegin(Button_HouseLevelUp)
  (params (FingerIndex :type ETouchIndex%20Enum :default "Touch1") (TouchedComponent :type Primitive%20Component%20Object%20Reference))
  ;[1 0 0] 연구_집레벨----------------- 나중에 해야함
  (Variables|Default|SetenableButton TouchedComponent))

(event OnInputTouchEnd(Button_ToMain)
  (params (FingerIndex :type ETouchIndex%20Enum :default "Touch1") (TouchedComponent :type Primitive%20Component%20Object%20Reference))
  ;[1 1 1] 오른쪽으로 이동
  (if (== TouchedComponent (Variables|Default|GetenableButton))
    (Collision|SetActorEnableCollision (Variables|Default|Getactor_HouseMenu) false)
    (Variables|Default|SetoriginalLocation (Transformation|GetActorLocation (Variables|Default|Getactor_HouseMenu)))
    (bind _인터페이스_이동 (Timeline|타임라인_0 PlayFromStart)
      (:Update
        (Transformation|SetActorLocation (Variables|Default|Getactor_HouseMenu) (+ (Math|Vector|MakeVector (* _인터페이스_이동 -288.0) 0.0 0.0) (Variables|Default|GetoriginalLocation)) false false))
      (:Finished
        (Collision|SetActorEnableCollision (Variables|Default|Getactor_HouseMenu) true)))))

(event OnInputTouchBegin(Button_ToMain)
  (params (FingerIndex :type ETouchIndex%20Enum :default "Touch1") (TouchedComponent :type Primitive%20Component%20Object%20Reference))
  ;[1 1 1] 오른쪽으로 이동
  (Variables|Default|SetenableButton TouchedComponent))

(event OnInputTouchEnd(Button_LabLevelUp)
  (params (FingerIndex :type ETouchIndex%20Enum :default "Touch1") (TouchedComponent :type Primitive%20Component%20Object%20Reference))
  ;[1 1 1] 연구 업그레이드
  (if (== TouchedComponent (Variables|Default|GetenableButton))
    (bind _ismax (CallFunction|ChecktheMAX))
    (if _ismax ; 연구 레벨이 최고 레벨인가
      (Class|WindowManager|CallOneButtonWindow(Message) (Variables|Default|Getactor_OneButtonWindow) "연구 레벨이 최고 상태입니다" self)
      (else
        (bind _isenough (CallFunction|ChecktheMoney true false))
        (if _isenough ; 돈이 충분한가
          (CallFunction|UpgradeLabLevel)
          (Class|WindowManager|RefreshTextBar(Message) (Variables|Default|Getactor_UserInfoBar))
          (else
            (Class|WindowManager|CallOneButtonWindow(Message) (Variables|Default|Getactor_OneButtonWindow) "돈부족" self)))))))

(event OnInputTouchBegin(Button_LabLevelUp)
  (params (FingerIndex :type ETouchIndex%20Enum :default "Touch1") (TouchedComponent :type Primitive%20Component%20Object%20Reference))
  ;[1 1 1] 연구 업그레이드
  (Variables|Default|SetenableButton TouchedComponent))

(event OnInputTouchEnd(Button_LabLevelDown)
  (params (FingerIndex :type ETouchIndex%20Enum :default "Touch1") (TouchedComponent :type Primitive%20Component%20Object%20Reference))
  ;[1 1 1] 연구 다운그레이드
  (if (== TouchedComponent (Variables|Default|GetenableButton))
    (if (<= (Variables|/Game/Blueprints/GameSetting/GameSaveData.GameSaveData_C|GetlabLevel (Variables|/Game/Blueprints/GameManager/GameManager.GameManager_C|GetgameSaveDataObject (Variables|Default|Getactor_GameManager))) 0) ; 연구 최저 레벨인지
      (Class|WindowManager|CallOneButtonWindow(Message) (Variables|Default|Getactor_OneButtonWindow) "연구 레벨이 최저 상태입니다" self)
      (else
        (bind _output_get (Variables|/Game/Blueprints/GameSetting/GameSaveData.GameSaveData_C|SetlabLevel (Variables|/Game/Blueprints/GameManager/GameManager.GameManager_C|GetgameSaveDataObject (Variables|Default|Getactor_GameManager)) (- (Variables|/Game/Blueprints/GameSetting/GameSaveData.GameSaveData_C|GetlabLevel (Variables|/Game/Blueprints/GameManager/GameManager.GameManager_C|GetgameSaveDataObject (Variables|Default|Getactor_GameManager))) 1)))
        (Class|WindowManager|CallOneButtonWindow(Message) (Variables|Default|Getactor_OneButtonWindow) (Utilities|String|Append "연구렙 " (Utilities|String|ToString(Integer) _output_get)) self)
        (SaveGame|SaveGametoSlot (Variables|/Game/Blueprints/GameManager/GameManager.GameManager_C|GetgameSaveDataObject (Variables|Default|Getactor_GameManager)) "GameSaveSlot1")
        (Class|WindowManager|RefreshTextBar(Message) (Variables|Default|Getactor_UserInfoBar))))))

(event OnInputTouchBegin(Button_LabLevelDown)
  (params (FingerIndex :type ETouchIndex%20Enum :default "Touch1") (TouchedComponent :type Primitive%20Component%20Object%20Reference))
  ;[1 1 1] 연구 다운그레이드
  (Variables|Default|SetenableButton TouchedComponent))

(event OnInputTouchEnd(Button_Hint)
  (params (FingerIndex :type ETouchIndex%20Enum :default "Touch1") (TouchedComponent :type Primitive%20Component%20Object%20Reference))
  ;[1 1 1] 연구_힌트보기
  (if (== TouchedComponent (Variables|Default|GetenableButton))
    (bind _all_opened (CallFunction|CheckAllNamedSword))
    (if _all_opened ; 모든 검 개방 여부 확인
      (Class|WindowManager|CallOneButtonWindow(Message) (Variables|Default|Getactor_OneButtonWindow) "이미 전부 개방" self)
      (else
        (bind _isenough (CallFunction|ChecktheMoney false true))
        (if _isenough ; 돈이 충분한지
          (bind (_개방되는_검 _하위_검 _소재_강화 _예리함_강화 _무게감_강화 _속성_강화) (CallFunction|OpenHint))
          (if (Utilities|Enum|NotEqual(Enum) _속성_강화 (Utilities|Text|MakeLiteralText "null")) ; 명검인지 아닌지(속성유무로 판단)
            (Class|WindowManager|CallOneButtonWindow(Message) (Variables|Default|Getactor_OneButtonWindow) (|힌트말만듦(명검)_2 _하위_검 _소재_강화 _예리함_강화 _무게감_강화 _속성_강화) self)
            (else
              (Class|WindowManager|CallOneButtonWindow(Message) (Variables|Default|Getactor_OneButtonWindow) (|힌트말만듦(일반)_2 _하위_검 _소재_강화 _예리함_강화 _무게감_강화 _속성_강화) self)))
          (SaveGame|SaveGametoSlot (Variables|/Game/Blueprints/GameManager/GameManager.GameManager_C|GetgameSaveDataObject (Variables|Default|Getactor_GameManager)) "GameSaveSlot1")
          (Class|WindowManager|RefreshTextBar(Message) (Variables|Default|Getactor_UserInfoBar))
          (else
            (Class|WindowManager|CallOneButtonWindow(Message) (Variables|Default|Getactor_OneButtonWindow) "돈 부족" self)))))))

(event OnInputTouchBegin(Button_Hint)
  (params (FingerIndex :type ETouchIndex%20Enum :default "Touch1") (TouchedComponent :type Primitive%20Component%20Object%20Reference))
  ;[1 1 1] 연구_힌트보기
  (Variables|Default|SetenableButton TouchedComponent))

(fn ConstructionScript)

(fn OpenHint
  (Variables|/Game/Blueprints/GameSetting/GameSaveData.GameSaveData_C|Setmoney (Variables|/Game/Blueprints/GameManager/GameManager.GameManager_C|GetgameSaveDataObject (Variables|Default|Getactor_GameManager)) (- (Variables|/Game/Blueprints/GameSetting/GameSaveData.GameSaveData_C|Getmoney (Variables|/Game/Blueprints/GameManager/GameManager.GameManager_C|GetgameSaveDataObject (Variables|Default|Getactor_GameManager))) 0.0))
  ;[1 1 1] 개방안된 검중에 당장 개방가능한검 리스트만들기
  (for (_array_element _array_index) (Variables|/Game/Blueprints/GameSetting/GameSaveData.GameSaveData_C|Getswordopen (Variables|/Game/Blueprints/GameManager/GameManager.GameManager_C|GetgameSaveDataObject (Variables|Default|Getactor_GameManager)))
    (if (not _array_element)
      (bind _returnvalue (Utilities|GetDataTableRow "/Game/Blueprints/SwordList.SwordList" (Utilities|String|StringToName (Utilities|String|ToString(Integer) _array_index)))
        (:then
          (bind _array_element_2 (Utilities|Array|ForEachLoopwithBreak (.하위검 _returnvalue) :!label _label)
            (:LoopBody
              (if (Utilities|Array|Get(acopy) (Variables|/Game/Blueprints/GameSetting/GameSaveData.GameSaveData_C|Getswordopen (Variables|/Game/Blueprints/GameManager/GameManager.GameManager_C|GetgameSaveDataObject (Variables|Default|Getactor_GameManager))) _array_element_2)
                (Utilities|Array|Add (LocalVariables|GetenableSwordList) _array_index)
                (goto _label Break))))))))
  ;[1 1 1] 리스트 중에서 한가지를 고르기
  (bind _output_get (LocalVariables|SetselectSword (Utilities|Array|Get(acopy) (LocalVariables|GetenableSwordList) (Math|Random|RandomInteger (Utilities|Array|Length (LocalVariables|GetenableSwordList))))))
  ;[1 1 1] 골라진 검의 하위검중 개방된검하나 고르기
  (bind _returnvalue_2 (Utilities|GetDataTableRow "/Game/Blueprints/SwordList.SwordList" (Utilities|String|StringToName (Utilities|String|ToString(Integer) _output_get)))
    (:then
      (LocalVariables|SetselectSwordName (.swordname _returnvalue_2))
      (for _array_element_3 (.하위검 _returnvalue_2)
        (if (Utilities|Array|Get(acopy) (Variables|/Game/Blueprints/GameSetting/GameSaveData.GameSaveData_C|Getswordopen (Variables|/Game/Blueprints/GameManager/GameManager.GameManager_C|GetgameSaveDataObject (Variables|Default|Getactor_GameManager))) _array_element_3)
          (Utilities|Array|Add (LocalVariables|GetselectSwordLowerList) _array_element_3)))
      (bind _output_get_2 (LocalVariables|SetselectLowerSword (Utilities|Array|Get(acopy) (LocalVariables|GetselectSwordLowerList) (Math|Random|RandomInteger (Utilities|Array|Length (LocalVariables|GetselectSwordLowerList))))))
      ;[1 1 1] 하위검에서 검의 개방조건 뽑아내기
      (bind _returnvalue_3 (Utilities|GetDataTableRow "/Game/Blueprints/SwordList.SwordList" (Utilities|String|StringToName (Utilities|String|ToString(Integer) _output_get_2)))
        (:then
          (bind (_array_element_4 _array_index_2) (Utilities|Array|ForEachLoopwithBreak (.개방되는검 _returnvalue_3) :!label _label_2)
            (:LoopBody
              (if (== (LocalVariables|GetselectSword) _array_element_4)
                (LocalVariables|Setindex _array_index_2)
                (goto _label_2 Break)))
            (:Completed
              (return (LocalVariables|GetselectSwordName) (.swordname _returnvalue_3) (/ (Utilities|Array|Get(acopy) (.개방조건 _returnvalue_3) (LocalVariables|Getindex)) 10000) (Math|Integer|%(Integer) (/ (Utilities|Array|Get(acopy) (.개방조건 _returnvalue_3) (LocalVariables|Getindex)) 100) 100) (Math|Integer|%(Integer) (Utilities|Array|Get(acopy) (.개방조건 _returnvalue_3) (LocalVariables|Getindex)) 100) (Utilities|Array|Get(acopy) (.개방조건_속성 _returnvalue_3) (LocalVariables|Getindex))))))))))

(fn ChecktheMAX
  (return (>= (Variables|/Game/Blueprints/GameSetting/GameSaveData.GameSaveData_C|GetlabLevel (Variables|/Game/Blueprints/GameManager/GameManager.GameManager_C|GetgameSaveDataObject (Variables|Default|Getactor_GameManager))) 10)))

(fn ChecktheMoney
  (params (FromUpgrade :type Boolean) (FromHint :type Boolean))
  (if FromUpgrade
    (return (>= (Variables|/Game/Blueprints/GameSetting/GameSaveData.GameSaveData_C|Getmoney (Variables|/Game/Blueprints/GameManager/GameManager.GameManager_C|GetgameSaveDataObject (Variables|Default|Getactor_GameManager))) (Utilities|Array|Get(acopy) (Variables|Default|GetlabUpgradePrice) (Variables|/Game/Blueprints/GameSetting/GameSaveData.GameSaveData_C|GetlabLevel (Variables|/Game/Blueprints/GameManager/GameManager.GameManager_C|GetgameSaveDataObject (Variables|Default|Getactor_GameManager))))))
    (elif FromHint
      (return (>= (Variables|/Game/Blueprints/GameSetting/GameSaveData.GameSaveData_C|Getmoney (Variables|/Game/Blueprints/GameManager/GameManager.GameManager_C|GetgameSaveDataObject (Variables|Default|Getactor_GameManager))) 0.0)))))

(fn UpgradeLabLevel
  (Variables|/Game/Blueprints/GameSetting/GameSaveData.GameSaveData_C|Setmoney (Variables|/Game/Blueprints/GameManager/GameManager.GameManager_C|GetgameSaveDataObject (Variables|Default|Getactor_GameManager)) (- (Variables|/Game/Blueprints/GameSetting/GameSaveData.GameSaveData_C|Getmoney (Variables|/Game/Blueprints/GameManager/GameManager.GameManager_C|GetgameSaveDataObject (Variables|Default|Getactor_GameManager))) (Utilities|Array|Get(acopy) (Variables|Default|GetlabUpgradePrice) (Variables|/Game/Blueprints/GameSetting/GameSaveData.GameSaveData_C|GetlabLevel (Variables|/Game/Blueprints/GameManager/GameManager.GameManager_C|GetgameSaveDataObject (Variables|Default|Getactor_GameManager))))))
  (bind _output_get (Variables|/Game/Blueprints/GameSetting/GameSaveData.GameSaveData_C|SetlabLevel (Variables|/Game/Blueprints/GameManager/GameManager.GameManager_C|GetgameSaveDataObject (Variables|Default|Getactor_GameManager)) (+ (Variables|/Game/Blueprints/GameSetting/GameSaveData.GameSaveData_C|GetlabLevel (Variables|/Game/Blueprints/GameManager/GameManager.GameManager_C|GetgameSaveDataObject (Variables|Default|Getactor_GameManager))) 1)))
  (Class|WindowManager|CallOneButtonWindow(Message) (Variables|Default|Getactor_OneButtonWindow) (Utilities|String|Append "연구렙 " (Utilities|String|ToString(Integer) _output_get)) self)
  (SaveGame|SaveGametoSlot (Variables|/Game/Blueprints/GameManager/GameManager.GameManager_C|GetgameSaveDataObject (Variables|Default|Getactor_GameManager)) "GameSaveSlot1"))

(fn CheckAllNamedSword
  (for _array_element (Variables|/Game/Blueprints/GameSetting/GameSaveData.GameSaveData_C|Getswordopen (Variables|/Game/Blueprints/GameManager/GameManager.GameManager_C|GetgameSaveDataObject (Variables|Default|Getactor_GameManager)))
    (if (not _array_element)
      (LocalVariables|SetisAllOpened false)))
  (return (LocalVariables|GetisAllOpened)))