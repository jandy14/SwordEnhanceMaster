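; UserInfoBar is an actor that displays the player's guild rank, experience and gold as text.
; On BeginPlay it hides itself and disables collision.
; A RefreshTextBar event reads GuildRank, Reliability (truncated to an integer and shown as Exp) and Money from the game manager's save data object, then writes them into three labelled text components.
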(event `self.ReceiveBeginPlay`
  ;[1 1 1] 초기화
  (`self.SetActorHiddenInGame` true)
  (`self.SetActorEnableCollision` false))

(event `/Game/Blueprints/WindowManager.RefreshTextBar`
  ;[1 1 1] Set TextBar 이벤트
  (`TextRenderComponent.K2_SetText` (`self.Text_GuildRank`) (`KismetTextLibrary.Conv_StringToText` (`KismetStringLibrary.Concat_StrStr` "Rank : " (`KismetStringLibrary.Conv_IntToString` (`/Game/Blueprints/GameSetting/GameSaveData.guildRank` (`/Game/Blueprints/GameManager/GameManager.gameSaveDataObject` (`self.actor_GameManager`)))))))
  (`TextRenderComponent.K2_SetText` (`self.Text_GuildReliability`) (`KismetTextLibrary.Conv_StringToText` (`KismetStringLibrary.Concat_StrStr` "Exp : " (`KismetStringLibrary.Conv_IntToString` (`KismetMathLibrary.FTrunc` (`/Game/Blueprints/GameSetting/GameSaveData.reliability` (`/Game/Blueprints/GameManager/GameManager.gameSaveDataObject` (`self.actor_GameManager`))))))))
  (`TextRenderComponent.K2_SetText` (`self.Text_GuildMoney`) (`KismetTextLibrary.Conv_StringToText` (`KismetStringLibrary.Concat_StrStr` "Gold : " (`KismetStringLibrary.Conv_IntToString` (`/Game/Blueprints/GameSetting/GameSaveData.money` (`/Game/Blueprints/GameManager/GameManager.gameSaveDataObject` (`self.actor_GameManager`)))) " G"))))

(fn `UserConstructionScript`)