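; OneButtonWindow is an actor that serves as a modal message window with a single confirm button.
; CallOneButtonWindow sets the message text, stores the calling scene actor, disables that actor's collision, then shows the window and enables its own collision.
; A touch that begins and ends on the button component hides the window and restores the scene's collision, so toggling actor collision gates touch input.
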(event `/Game/Blueprints/WindowManager.CallOneButtonWindow`
  (params (Text :type String) (Scene :type "Actor Object Reference"))
  ;[1 1 1] 윈도우 호출
  (set `self.attachToScene` Scene)
  (`TextRenderComponent.K2_SetText` (`self.MainText`) (`KismetTextLibrary.Conv_StringToText` Text))
  (`self.SetActorEnableCollision` (`self.attachToScene`) false)
  (`self.SetActorHiddenInGame` false)
  (`self.SetActorEnableCollision` true))

(event `self.Button.OnInputTouchEnd`
  (params (FingerIndex :type "ETouchIndex Enum" :default "Touch1") (TouchedComponent :type "PrimitiveComponent Object Reference"))
  ;[1 1 1] 확인 버튼 이벤트
  (if (== TouchedComponent (`self.enableButton`))
    (`self.SetActorEnableCollision` false)
    (`self.SetActorHiddenInGame` true)
    (`self.SetActorEnableCollision` (`self.attachToScene`) true)))

(event `self.Button.OnInputTouchBegin`
  (params (FingerIndex :type "ETouchIndex Enum" :default "Touch1") (TouchedComponent :type "PrimitiveComponent Object Reference"))
  ;[1 1 1] 확인 버튼 이벤트
  (set `self.enableButton` TouchedComponent))

(fn `UserConstructionScript`)