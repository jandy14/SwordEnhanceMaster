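; Sprite-based weapon inventory popup, opened for picking a sword to enhance or for selling swords at the store.
; Slots show saved sword data, with a detail pane for the selected one.
; Touch dragging scrolls the panel horizontally, recycling a fixed slot pool by wrapping off-edge slots and reindexing them.
; Select returns the index to the calling scene, whose collision is off meanwhile; sell mode tracks checkboxes and delegates pricing and sales to the weapon menu.
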(event OnInputTouchEnd(SelectButton)
  (params (FingerIndex :type ETouchIndex%20Enum :default "Touch1") (TouchedComponent :type Primitive%20Component%20Object%20Reference))
  ;[1 1 1] 선택/판매 버튼 이벤트
  (if (== TouchedComponent (Variables|Default|GetenableButton))
    (if (Variables|Default|GetisCheckable)
      (Class|InventoryManager|SellWeapons(Message) (Variables|Default|Getactor_WeaponMenu))
      ;[1 1 1] 인벤토리 닫기
      (Rendering|SetActorHiddenInGame true :!label _label)
      (Collision|SetActorEnableCollision false)
      (|아이템슬롯비활성화)
      (Collision|SetActorEnableCollision (Variables|Default|Getactor_AttachToScene) true)
      (Variables|Default|Setvalue 15)
      (Variables|Default|SetisCheckable false)
      (elif (Variables|Default|GetisSelected)
        (Class|InventoryManager|SelectItem(Message) (Variables|Default|Getactor_AttachToScene) (Variables|Default|GetselectIndex)) ; 선택 버튼
        (goto _label)))))

(event OnInputTouchBegin(SelectButton)
  (params (FingerIndex :type ETouchIndex%20Enum :default "Touch1") (TouchedComponent :type Primitive%20Component%20Object%20Reference))
  ;[1 1 1] 선택/판매 버튼 이벤트
  (Variables|Default|SetenableButton TouchedComponent))

(event OnInputTouchBegin(CloseButton_Sprite)
  (params (FingerIndex :type ETouchIndex%20Enum :default "Touch1") (TouchedComponent :type Primitive%20Component%20Object%20Reference))
  ;[1 1 1] 인벤토리 닫기
  (Variables|Default|SetenableButton TouchedComponent))

(event OnInputTouchEnd(CloseButton_Sprite)
  (params (FingerIndex :type ETouchIndex%20Enum :default "Touch1") (TouchedComponent :type Primitive%20Component%20Object%20Reference))
  ;[1 1 1] 인벤토리 닫기
  (if (== TouchedComponent (Variables|Default|GetenableButton))
    (Rendering|SetActorHiddenInGame true)
    (Collision|SetActorEnableCollision false)
    (|아이템슬롯비활성화)
    (Collision|SetActorEnableCollision (Variables|Default|Getactor_AttachToScene) true)
    (Variables|Default|Setvalue 15)
    (Variables|Default|SetisCheckable false)))

(event Custom|Set%20Slot%20Location
  ;[1 1 1] Set Slot Location 이벤트
  (for _array_element (Variables|Default|Getarray_Slot)
    (|왼쪽으로넘어간슬롯관리 _array_element
      (:true
        _)
      (:false
        (|오른쪽으로넘어간슬롯관리 _array_element)))
    (CallFunction|RefreshSlot _array_element)
    (CallFunction|ChecktheCheckBox _array_element)))

(event Custom|Refresh%20Slot
  (params (slot :type Slot%20Object%20Reference))
  ;[1 1 1] 슬롯 정보 새로고침
  (Variables|Default|Setactor_Slot slot)
  (if (>= (Variables|/Game/Blueprints/Inventory/Slot.Slot_C|Getindex (Variables|Default|Getactor_Slot)) 0) ; 유효한 슬롯인가
    (CallFunction|SetSwordImage (Variables|Default|Getactor_Slot))
    (CallFunction|SetEnhancementText (Variables|Default|Getactor_Slot))))

(event EventChecktheWeapon
  (params (index :type Integer) (slot :type Slot%20Object%20Reference))
  (bind _array_checkedweapon (Variables|Default|Getarray_CheckedWeapon))
  (bind _item (Utilities|Array|Get(acopy) _array_checkedweapon index))
  ;[1 1 1] Check the Weapon 이벤트
  (Utilities|Array|SetArrayElem (Variables|Default|Getarray_CheckedWeapon) index (not _item) true)
  (CallFunction|ChecktheCheckBox slot)
  (Class|InventoryManager|CalculateWeaponPrice(Message) (Variables|Default|Getactor_WeaponMenu) index _item))

(event EventShowInventory
  (params (SceneFrom :type Actor%20Object%20Reference) (FromEnhancement :type Boolean) (FromWeaponStore :type Boolean))
  ;[1 1 1] 무기 인벤토리 활성화
  (|인벤토리인지상점인지판단 FromEnhancement FromWeaponStore)
  (bind _output_get (Variables|Default|Setactor_AttachToScene SceneFrom))
  (Collision|SetActorEnableCollision _output_get false)
  (Rendering|SetActorHiddenInGame false)
  (Collision|SetActorEnableCollision true)
  (Variables|Default|SetselectIndex -1)
  (|아이템정보창초기화)
  (|아이템슬롯활성화)
  (|배열초기화)
  (Class|InventoryManager|SetItemSlot(Message) self))

(event EventActorOnInputTouchEnd
  (params (FingerIndex :type ETouchIndex%20Enum :default "Touch1"))
  (bind _returnvalue (Game|GetPlayerController 0))
  (bind (_locationx _locationy) (Game|Player|GetMousePosition _returnvalue))
  ;[1 1 1] 드래그 시작/종료
  (Variables|Default|SetisPressed false)
  (Variables|Default|Setvector_MousePosition (Math|Vector|MakeVector _locationx _locationy -23.5)))

(event EventActorOnInputTouchBegin
  (params (FingerIndex :type ETouchIndex%20Enum :default "Touch1"))
  (bind _returnvalue (Game|GetPlayerController 0))
  (bind (_locationx _locationy) (Game|Player|GetMousePosition _returnvalue))
  ;[1 1 1] 드래그 시작/종료
  (Variables|Default|SetisPressed true)
  (Variables|Default|Setvector_MousePosition (Math|Vector|MakeVector _locationx _locationy -23.5)))

(event EventSetItemSlot
  ;[1 1 1] Set Item Slot 이벤트
  (for _array_element (Variables|Default|Getarray_Slot)
    (CallFunction|SetSwordImage _array_element)
    (CallFunction|SetEnhancementText _array_element)))

(event EventBeginPlay
  ;[1 1 1] 초기화
  (Rendering|SetActorHiddenInGame true)
  (Collision|SetActorEnableCollision false))

(event EventSelectItem
  (params (Index :type Integer))
  (bind _selectindex (Variables|Default|GetselectIndex))
  (bind _actor_gamemanager (Variables|Default|Getactor_GameManager))
  (bind _gamesavedataobject (Variables|/Game/Blueprints/GameManager/GameManager.GameManager_C|GetgameSaveDataObject _actor_gamemanager))
  (bind _swordinfo (Variables|/Game/Blueprints/GameSetting/GameSaveData.GameSaveData_C|GetswordInfo _gamesavedataobject))
  (bind _item (Utilities|Array|Get(acopy) _swordinfo _selectindex))
  (bind (_swordname _swordnumber _소재강화 _예리함강화 _무게감강화 _속성강화) (Utilities|Struct|BreakSwordInfo _item))
  ;[1 1 1] 무기 정보 출력
  (|SetImage Index)
  (|SetName _swordname _속성강화)
  (|SetEnhancementValue _소재강화 _예리함강화 _무게감강화))

(event EventTick
  (params (DeltaSeconds :type Float%20%28single-precision%29))
  (bind _returnvalue (Game|GetPlayerController 0))
  (bind _actor_panel (Variables|Default|Getactor_Panel))
  (bind _actor_panel_2 (Variables|Default|Getactor_Panel))
  (bind _locationx (Game|Player|GetMousePosition _returnvalue))
  (bind _returnvalue_2 (Transformation|GetActorLocation _actor_panel))
  (bind _returnvalue_3 (Transformation|GetActorLocation _actor_panel_2))
  (bind (_x _y _z) (Math|Vector|BreakVector _returnvalue_3))
  (bind _returnvalue_4 (Math|Vector|MakeVector _locationx 0.0 -23.5))
  (bind (_x_2 _y_2 _z_2) (Math|Vector|BreakVector _returnvalue_2))
  ;[1 1 1] 드래그 이벤트
  (if (Variables|Default|GetisPressed) ; 클릭중인가
    (bind _disable (CallFunction|ChecktheEnableArea))
    (if _disable
      (Variables|Default|SetisPressed false)
      (elif (or (> (- (.LocationX (Game|Player|GetMousePosition (Game|GetPlayerController 0))) (.X (Math|Vector|BreakVector (Variables|Default|Getvector_MousePosition)))) 1.0) (< (- (.LocationX (Game|Player|GetMousePosition (Game|GetPlayerController 0))) (.X (Math|Vector|BreakVector (Variables|Default|Getvector_MousePosition)))) -1.0)) ; 드래그가 되었는가
        (if (> _x_2 0.0) ; 슬롯 이동범위 체크
          (Transformation|SetActorLocation (Variables|Default|Getactor_Panel) (Math|Vector|MakeVector 0.0 _y_2 _z_2) false false)
          (Variables|Default|Setvector_MousePosition _returnvalue_4)
          (else
            (Transformation|SetActorLocation (Variables|Default|Getactor_Panel) (Math|Vector|MakeVector (+ (- (.LocationX (Game|Player|GetMousePosition (Game|GetPlayerController 0))) (.X (Math|Vector|BreakVector (Variables|Default|Getvector_MousePosition)))) _x) _y _z) false false)
            (Variables|Default|Setvector_MousePosition _returnvalue_4)
            (CallFunction|SetSlotLocation)))))))

(fn ConstructionScript)

(fn SetSwordImage
  (params (Slot :type Slot%20Object%20Reference))
  (LocalVariables|SettmpSlot Slot)
  (if (< (Variables|/Game/Blueprints/Inventory/Slot.Slot_C|Getindex (LocalVariables|GettmpSlot)) (Utilities|Array|Length (Variables|/Game/Blueprints/GameSetting/GameSaveData.GameSaveData_C|GetswordInfo (Variables|/Game/Blueprints/GameManager/GameManager.GameManager_C|GetgameSaveDataObject (Variables|Default|Getactor_GameManager))))) ; 표시할 아이템이 있는가
    (Rendering|Components|Sprite|SetSprite (Variables|/Game/Blueprints/Inventory/Slot.Slot_C|GetSwordImage (LocalVariables|GettmpSlot)) (Utilities|Array|Get(acopy) (Variables|/Game/Blueprints/GameManager/GameManager.GameManager_C|Getarray_SwordSprite (Variables|Default|Getactor_GameManager)) (Math|Conversions|ToInteger(Byte) (Utilities|String|ToString(Name) (.swordNumber (Utilities|Struct|BreakSwordInfo (Utilities|Array|Get(acopy) (Variables|/Game/Blueprints/GameSetting/GameSaveData.GameSaveData_C|GetswordInfo (Variables|/Game/Blueprints/GameManager/GameManager.GameManager_C|GetgameSaveDataObject (Variables|Default|Getactor_GameManager))) (Variables|/Game/Blueprints/Inventory/Slot.Slot_C|Getindex (LocalVariables|GettmpSlot)))))))))
    (Transformation|SetWorldScale3D (Variables|/Game/Blueprints/Inventory/Slot.Slot_C|GetSwordImage (LocalVariables|GettmpSlot)) "100.000000,100.000000,100.000000")
    (else
      (Rendering|Components|Sprite|SetSprite (Variables|/Game/Blueprints/Inventory/Slot.Slot_C|GetSwordImage (LocalVariables|GettmpSlot)) "/Game/Sprites/OrthoWidth-144/ItemSlotPanel_Sprite.ItemSlotPanel_Sprite")
      (Transformation|SetWorldScale3D (Variables|/Game/Blueprints/Inventory/Slot.Slot_C|GetSwordImage (LocalVariables|GettmpSlot)) "1.000000,1.000000,1.000000"))))

(fn SetEnhancementText
  (params (slot :type Slot%20Object%20Reference))
  (LocalVariables|SettmpSlot slot)
  (if (< (Variables|/Game/Blueprints/Inventory/Slot.Slot_C|Getindex (LocalVariables|GettmpSlot)) (Utilities|Array|Length (Variables|/Game/Blueprints/GameSetting/GameSaveData.GameSaveData_C|GetswordInfo (Variables|/Game/Blueprints/GameManager/GameManager.GameManager_C|GetgameSaveDataObject (Variables|Default|Getactor_GameManager))))) ; 표시할 아이템이 있는가
    (Rendering|Components|TextRender|SetText (Variables|/Game/Blueprints/Inventory/Slot.Slot_C|GetText (LocalVariables|GettmpSlot)) (Utilities|Text|ToText(String) (Utilities|String|Append "+" (Utilities|String|ToString(Integer) (+ (.소재강화 (Utilities|Struct|BreakSwordInfo (Utilities|Array|Get(acopy) (Variables|/Game/Blueprints/GameSetting/GameSaveData.GameSaveData_C|GetswordInfo (Variables|/Game/Blueprints/GameManager/GameManager.GameManager_C|GetgameSaveDataObject (Variables|Default|Getactor_GameManager))) (Variables|/Game/Blueprints/Inventory/Slot.Slot_C|Getindex (LocalVariables|GettmpSlot))))) (.예리함강화 (Utilities|Struct|BreakSwordInfo (Utilities|Array|Get(acopy) (Variables|/Game/Blueprints/GameSetting/GameSaveData.GameSaveData_C|GetswordInfo (Variables|/Game/Blueprints/GameManager/GameManager.GameManager_C|GetgameSaveDataObject (Variables|Default|Getactor_GameManager))) (Variables|/Game/Blueprints/Inventory/Slot.Slot_C|Getindex (LocalVariables|GettmpSlot))))) (.무게감강화 (Utilities|Struct|BreakSwordInfo (Utilities|Array|Get(acopy) (Variables|/Game/Blueprints/GameSetting/GameSaveData.GameSaveData_C|GetswordInfo (Variables|/Game/Blueprints/GameManager/GameManager.GameManager_C|GetgameSaveDataObject (Variables|Default|Getactor_GameManager))) (Variables|/Game/Blueprints/Inventory/Slot.Slot_C|Getindex (LocalVariables|GettmpSlot))))) (Math|Conversions|ToInteger(Boolean) (Utilities|Enum|NotEqual(Enum) (.속성강화 (Utilities|Struct|BreakSwordInfo (Utilities|Array|Get(acopy) (Variables|/Game/Blueprints/GameSetting/GameSaveData.GameSaveData_C|GetswordInfo (Variables|/Game/Blueprints/GameManager/GameManager.GameManager_C|GetgameSaveDataObject (Variables|Default|Getactor_GameManager))) (Variables|/Game/Blueprints/Inventory/Slot.Slot_C|Getindex (LocalVariables|GettmpSlot))))) (Utilities|Text|MakeLiteralText "null"))))))))
    (else
      (Rendering|Components|TextRender|SetText (Variables|/Game/Blueprints/Inventory/Slot.Slot_C|GetText (LocalVariables|GettmpSlot)) (Utilities|Text|MakeLiteralText " ")))))

(fn ChecktheEnableArea
  (bind _returnvalue (Game|GetPlayerController 0))
  (bind _worldlocation (Game|Player|ConvertMouseLocationToWorldSpace _returnvalue))
  (bind (_x _y _z) (Math|Vector|BreakVector _worldlocation))
  (return (or (or (>= _x 1.2e+02) (<= _x -1.2e+02)) (or (>= _z 72.0) (<= _z -142.0)))))

(fn ResetSlotLocation
  (params (slot :type Slot%20Object%20Reference) (index :type Integer))
  (LocalVariables|SetlocalIndex index)
  (LocalVariables|Setlocation_PositionX (+ (* (/ (LocalVariables|GetlocalIndex) 2) 36.0) -92.0))
  (if (== (Math|Integer|%(Integer) (LocalVariables|GetlocalIndex) 2) 0)
    (LocalVariables|Setlocation_PositionZ -8e+01)
    (else
      (LocalVariables|Setlocation_PositionZ -116.0)))
  (Transformation|SetActorLocation slot (Math|Vector|MakeVector (LocalVariables|Getlocation_PositionX) 155.0 (LocalVariables|Getlocation_PositionZ)) false true))

(fn ChecktheCheckBox
  (params (slot :type Slot%20Object%20Reference))
  (LocalVariables|SettmpSlot slot)
  (Development|SetHiddeninGame (Variables|/Game/Blueprints/Inventory/Slot.Slot_C|GetCheckBox (LocalVariables|GettmpSlot)) (not (Utilities|Array|Get(acopy) (Variables|Default|Getarray_CheckedWeapon) (Variables|/Game/Blueprints/Inventory/Slot.Slot_C|Getindex (LocalVariables|GettmpSlot)))) false))