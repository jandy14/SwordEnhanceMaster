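; Touch-selectable item slot actor shared by the weapon inventory and weapon store, hidden and without collision at BeginPlay.
; Collider touch begin and end update both owner actors' pressed state and pass them the mouse position with a fixed Z for each.
; A release on the component first pressed sends the slot index to check the weapon if the inventory is checkable, otherwise to select the item in both actors.
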(event `self.ReceiveBeginPlay`
  (`SceneComponent.SetHiddenInGame` (`self.ItemSlot`) true true)
  (`self.SetActorEnableCollision` self false))

(event `self.Collider.OnInputTouchEnd`
  (params (FingerIndex :type "ETouchIndex Enum" :default "Touch1") (TouchedComponent :type "PrimitiveComponent Object Reference"))
  (bind (_locationx _locationy) (`PlayerController.GetMousePosition` (`GameplayStatics.GetPlayerController` 0)))
  (bind (_locationx_2 _locationy_2) (`PlayerController.GetMousePosition` (`GameplayStatics.GetPlayerController` 0)))
  (set `/Game/Blueprints/Inventory/WeaponInventory.isPressed` false (`self.actor_WeaponInventory`))
  (set `/Game/Blueprints/Guild/WeaponStore.isPressed` false (`self.actor_WeaponStore`))
  (set `/Game/Blueprints/Guild/WeaponStore.vector_MousePosition` (`KismetMathLibrary.MakeVector` _locationx_2 _locationy_2 26.0) (`self.actor_WeaponStore`))
  (set `/Game/Blueprints/Inventory/WeaponInventory.vector_MousePosition` (`KismetMathLibrary.MakeVector` _locationx _locationy -23.5) (`self.actor_WeaponInventory`))
  (if (== TouchedComponent (`self.button`))
    (if (`/Game/Blueprints/Inventory/WeaponInventory.isCheckable` (`self.actor_WeaponInventory`))
      (message `/Game/Blueprints/Inventory/InventoryManager.CheckTheWeapon` (`self.actor_WeaponInventory`) (`self.index`) self)
      (else
        (message `/Game/Blueprints/Inventory/InventoryManager.SelectItem` (`self.actor_WeaponInventory`) (`self.index`))
        (message `/Game/Blueprints/Inventory/InventoryManager.SelectItem` (`self.actor_WeaponStore`) (`self.index`))))))

(event `self.Collider.OnInputTouchBegin`
  (params (FingerIndex :type "ETouchIndex Enum" :default "Touch1") (TouchedComponent :type "PrimitiveComponent Object Reference"))
  (bind (_locationx _locationy) (`PlayerController.GetMousePosition` (`GameplayStatics.GetPlayerController` 0)))
  (bind (_locationx_2 _locationy_2) (`PlayerController.GetMousePosition` (`GameplayStatics.GetPlayerController` 0)))
  (set `self.button` TouchedComponent)
  (set `/Game/Blueprints/Inventory/WeaponInventory.isPressed` true (`self.actor_WeaponInventory`))
  (set `/Game/Blueprints/Guild/WeaponStore.isPressed` true (`self.actor_WeaponStore`))
  (set `/Game/Blueprints/Guild/WeaponStore.vector_MousePosition` (`KismetMathLibrary.MakeVector` _locationx _locationy 26.0) (`self.actor_WeaponStore`))
  (set `/Game/Blueprints/Inventory/WeaponInventory.vector_MousePosition` (`KismetMathLibrary.MakeVector` _locationx_2 _locationy_2 -23.5) (`self.actor_WeaponInventory`)))

(fn `UserConstructionScript`)