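; IngredientSlot is a touchable slot in the ingredient inventory that selects its item by index.
; Touch begin and end on its Collider update the inventory actor's pressed flag and pointer position, read from the mouse with a fixed Z.
; Touch begin stores the touched component and prints the index for debugging.
; Touch end calls SelectIngredientItemMessage with the index only if the same component is released.
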(event `self.Collider.OnInputTouchEnd`
  (params (FingerIndex :type "ETouchIndex Enum" :default "Touch1") (TouchedComponent :type "PrimitiveComponent Object Reference"))
  (bind (_locationx _locationy) (`PlayerController.GetMousePosition` (`GameplayStatics.GetPlayerController` 0)))
  (set `/Game/Blueprints/Inventory/IngredientInventory.isPressed` false (`self.actor_IngredientInventory`))
  (set `/Game/Blueprints/Inventory/IngredientInventory.vector_MousePosition` (`KismetMathLibrary.MakeVector` _locationx _locationy -23.5) (`self.actor_IngredientInventory`))
  (if (== TouchedComponent (`self.button`))
    (message `/Game/Blueprints/Inventory/InventoryManager.SelectIngredientItem` (`self.actor_IngredientInventory`) (`self.index`))))

(event `self.Collider.OnInputTouchBegin`
  (params (FingerIndex :type "ETouchIndex Enum" :default "Touch1") (TouchedComponent :type "PrimitiveComponent Object Reference"))
  (bind (_locationx _locationy) (`PlayerController.GetMousePosition` (`GameplayStatics.GetPlayerController` 0)))
  (set `self.button` TouchedComponent)
  (set `/Game/Blueprints/Inventory/IngredientInventory.isPressed` true (`self.actor_IngredientInventory`))
  (set `/Game/Blueprints/Inventory/IngredientInventory.vector_MousePosition` (`KismetMathLibrary.MakeVector` _locationx _locationy -23.5) (`self.actor_IngredientInventory`))
  (`KismetSystemLibrary.PrintString` (`KismetStringLibrary.Conv_IntToString` (`self.index`))))

(fn `UserConstructionScript`)