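; Ingredient inventory actor: a sprite-based popup where the player picks a common or rare ingredient for the scene that opened it.
; Touch-dragging slides the panel within clamped bounds, recycling a small pool of slot actors by wrapping positions and re-indexing them across 18 entries.
; Slots show sprites and counts from save data; selection previews the item, disables Select at zero stock, and confirming messages the calling scene, then closes and resets the panel.
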(event OnInputTouchEnd(Button_Select)
  (params (FingerIndex :type ETouchIndex%20Enum :default "Touch1") (TouchedComponent :type Primitive%20Component%20Object%20Reference))
  ;[1 1 1] 선택 버튼 이벤트
  (if (== TouchedComponent (Variables|Default|GetenableButton))
    (if (Variables|Default|GetisSelected)
      (Class|InventoryManager|SelectIngredient(Message) (Variables|디폴트|Getactor_AttachToScene) (Variables|Default|GetselectIndex))
      ;[1 1 1] 인벤토리 닫기
      (Rendering|SetActorHiddenInGame true)
      (Collision|SetActorEnableCollision false)
      (Collision|SetActorEnableCollision (Variables|디폴트|Getactor_AttachToScene) true)
      (Transformation|SetActorLocation (Variables|Default|Getpanel) "0,340.000000,-97.000000" false false)
      (|아이템슬롯비활성화)
      (Rendering|Components|Sprite|SetSprite (Variables|Default|GetIngredientImage) "/Game/Sprites/OrthoWidth-144/ItemSlotPanel_Sprite.ItemSlotPanel_Sprite")
      (Transformation|SetWorldScale3D (Variables|Default|GetIngredientImage) "0.050000,0.050000,0.050000")
      (Variables|Default|Setvalue 7))))

(event OnInputTouchBegin(Button_Select)
  (params (FingerIndex :type ETouchIndex%20Enum :default "Touch1") (TouchedComponent :type Primitive%20Component%20Object%20Reference))
  ;[1 1 1] 선택 버튼 이벤트
  (Variables|Default|SetenableButton TouchedComponent))

(event OnInputTouchEnd(CloseButton_Sprite)
  (params (FingerIndex :type ETouchIndex%20Enum :default "Touch1") (TouchedComponent :type Primitive%20Component%20Object%20Reference))
  ;[1 1 1] 인벤토리 닫기
  (if (== TouchedComponent (Variables|Default|GetenableButton))
    (Rendering|SetActorHiddenInGame true)
    (Collision|SetActorEnableCollision false)
    (Collision|SetActorEnableCollision (Variables|디폴트|Getactor_AttachToScene) true)
    (Transformation|SetActorLocation (Variables|Default|Getpanel) "0,340.000000,-97.000000" false false)
    (|아이템슬롯비활성화)
    (Rendering|Components|Sprite|SetSprite (Variables|Default|GetIngredientImage) "/Game/Sprites/OrthoWidth-144/ItemSlotPanel_Sprite.ItemSlotPanel_Sprite")
    (Transformation|SetWorldScale3D (Variables|Default|GetIngredientImage) "0.050000,0.050000,0.050000")
    (Variables|Default|Setvalue 7)))

(event OnInputTouchBegin(CloseButton_Sprite)
  (params (FingerIndex :type ETouchIndex%20Enum :default "Touch1") (TouchedComponent :type Primitive%20Component%20Object%20Reference))
  ;[1 1 1] 인벤토리 닫기
  (Variables|Default|SetenableButton TouchedComponent))

(event Custom|Refresh%20Slot
  (params (slot :type Ingredient%20Slot%20Object%20Reference))
  ;[1 1 1] Refresh Slot
  (Variables|Default|SetaSlot slot)
  (if (and (>= (Variables|/Game/Blueprints/Inventory/IngredientSlot.IngredientSlot_C|Getindex (Variables|Default|GetaSlot)) 0) (< (Variables|/Game/Blueprints/Inventory/IngredientSlot.IngredientSlot_C|Getindex (Variables|Default|GetaSlot)) 18)) ; 유효한 슬롯인가
    (CallFunction|SetIngredientImage (Variables|Default|GetaSlot))
    (CallFunction|SetIngredientCount (Variables|Default|GetaSlot))))

(event Custom|Set%20Slot%20Location
  ;[1 1 1] Set Slot Location
  (for _array_element (Variables|Default|Getarray_Slot)
    (|왼쪽으로넘어간슬롯관리 _array_element
      (:true
        _)
      (:false
        (|오른쪽으로넘어간슬롯관리 _array_element)))
    (CallFunction|RefreshSlot _array_element)))

(event EventActorOnInputTouchEnd
  (params (FingerIndex :type ETouchIndex%20Enum :default "Touch1"))
  (bind _returnvalue (Game|GetPlayerController 0))
  (bind (_locationx _locationy) (Game|Player|GetMousePosition _returnvalue))
  ;[1 1 1] 드래그 시작/종료
  (Variables|Default|SetisPressed false)
  (Variables|Default|Setvector_MousePosition (Math|Vector|MakeVector _locationx _locationy -23.5)))

(event EventActorOnInputTouchBegin
  (params (FingerIndex :type ETouchIndex%20Enum :default "Touch1"))
  (bind _returnvalue (Game|GetPlayerController 0))
  (bind (_locationx _locationy) (Game|Player|GetMousePosition _returnvalue))
  ;[1 1 1] 드래그 시작/종료
  (Variables|Default|SetisPressed true)
  (Variables|Default|Setvector_MousePosition (Math|Vector|MakeVector _locationx _locationy -23.5)))

(event EventSetIngredientItemSlot
  (params (Index :type Integer))
  ;[1 1 1] Set Ingredient Item Slot 이벤트
  (for _array_element (Variables|Default|Getarray_Slot)
    (CallFunction|SetIngredientImage _array_element)
    (CallFunction|SetIngredientCount _array_element)))

(event EventSelectIngredientItem
  (params (Index :type Integer))
  ;[1 1 1] 소재 클릭 이벤트
  (|SetImage Index)
  (CallFunction|ChecktheCount))

(event EventBeginPlay
  ;[1 1 1] 비활성화
  (Rendering|SetActorHiddenInGame true)
  (Collision|SetActorEnableCollision false))

(event EventTick
  (params (DeltaSeconds :type Float%20%28single-precision%29))
  (bind _returnvalue (Game|GetPlayerController 0))
  (bind _panel (Variables|Default|GetPanel))
  (bind _panel_2 (Variables|Default|GetPanel))
  (bind _panel_3 (Variables|Default|GetPanel))
  (bind _locationx (Game|Player|GetMousePosition _returnvalue))
  (bind _returnvalue_2 (Transformation|GetActorLocation _panel_2))
  (bind _returnvalue_3 (Transformation|GetActorLocation _panel))
  (bind _returnvalue_4 (Transformation|GetActorLocation _panel_3))
  (bind (_x _y _z) (Math|Vector|BreakVector _returnvalue_4))
  (bind _returnvalue_5 (Math|Vector|MakeVector _locationx 0.0 -23.5))
  (bind (_x_2 _y_2 _z_2) (Math|Vector|BreakVector _returnvalue_3))
  (bind (_x_3 _y_3 _z_3) (Math|Vector|BreakVector _returnvalue_2))
  ;[1 1 1] 드래그 이벤트
  (if (Variables|Default|GetisPressed) ; 클릭중인가
    (bind _disable (CallFunction|ChecktheEnableArea))
    (if _disable
      (Variables|Default|SetisPressed false)
      (elif (or (> (- (.LocationX (Game|Player|GetMousePosition (Game|GetPlayerController 0))) (.X (Math|Vector|BreakVector (Variables|Default|Getvector_MousePosition)))) 1.0) (< (- (.LocationX (Game|Player|GetMousePosition (Game|GetPlayerController 0))) (.X (Math|Vector|BreakVector (Variables|Default|Getvector_MousePosition)))) -1.0)) ; 드래그가 되었는가
        (if (> _x_3 0.0) ; 슬롯 이동범위 체크
          (Transformation|SetActorLocation (Variables|Default|GetPanel) (Math|Vector|MakeVector 0.0 _y_3 _z_3) false false)
          (Variables|Default|Setvector_MousePosition _returnvalue_5)
          (elif (< _x_3 -426.0)
            (Transformation|SetActorLocation (Variables|Default|GetPanel) (Math|Vector|MakeVector -426.0 _y_2 _z_2) false false)
            (Variables|Default|Setvector_MousePosition _returnvalue_5)
            (else
              (Transformation|SetActorLocation (Variables|Default|GetPanel) (Math|Vector|MakeVector (+ (- (.LocationX (Game|Player|GetMousePosition (Game|GetPlayerController 0))) (.X (Math|Vector|BreakVector (Variables|Default|Getvector_MousePosition)))) _x) _y _z) false false)
              (Variables|Default|Setvector_MousePosition _returnvalue_5)
              (CallFunction|SetSlotLocation))))))))

(event EventShowIngredientInventory
  (params (SceneFrom :type Actor%20Object%20Reference))
  ;[1 1 1] 재료창 활성화
  (Variables|디폴트|Setactor_AttachToScene SceneFrom)
  (Collision|SetActorEnableCollision (Variables|디폴트|Getactor_AttachToScene) false)
  (Rendering|SetActorHiddenInGame false)
  (Collision|SetActorEnableCollision true)
  (Rendering|Components|TextRender|SetText (Variables|Default|GetIngredientName) (Utilities|Text|MakeLiteralText " "))
  (|아이템슬롯활성화)
  (|레어소재체크
    (:Completed
      (Class|InventoryManager|SetIngredientItemSlot(Message) self (Variables|Default|GetingredientType)))))

(fn ConstructionScript)

(fn SetIngredientImage
  (params (slot :type Ingredient%20Slot%20Object%20Reference))
  (LocalVariables|SettmpSlot slot)
  (if (< (Variables|/Game/Blueprints/Inventory/IngredientSlot.IngredientSlot_C|Getindex (LocalVariables|GettmpSlot)) 9) ; 일반 소재인가
    (Rendering|Components|Sprite|SetSprite (Variables|/Game/Blueprints/Inventory/IngredientSlot.IngredientSlot_C|GetIngredientImage (LocalVariables|GettmpSlot)) (Utilities|Array|Get(acopy) (Variables|/Game/Blueprints/GameManager/GameManager.GameManager_C|Getarray_IngredientSprite (Variables|Default|Getactor_GameManager)) (Variables|/Game/Blueprints/Inventory/IngredientSlot.IngredientSlot_C|Getindex (LocalVariables|GettmpSlot))))
    (Transformation|SetWorldScale3D (Variables|/Game/Blueprints/Inventory/IngredientSlot.IngredientSlot_C|GetIngredientImage (LocalVariables|GettmpSlot)) "100.000000,100.000000,100.000000")
    (elif (!= (Utilities|Array|Get(acopy) (Variables|Default|GetrareIndex) (Variables|/Game/Blueprints/Inventory/IngredientSlot.IngredientSlot_C|Getindex (LocalVariables|GettmpSlot))) 0) ; 레어 소재가 있는가
      (Rendering|Components|Sprite|SetSprite (Variables|/Game/Blueprints/Inventory/IngredientSlot.IngredientSlot_C|GetIngredientImage (LocalVariables|GettmpSlot)) (Utilities|Array|Get(acopy) (Variables|/Game/Blueprints/GameManager/GameManager.GameManager_C|Getarray_IngredientSprite (Variables|Default|Getactor_GameManager)) (Utilities|Array|Get(acopy) (Variables|Default|GetrareIndex) (Variables|/Game/Blueprints/Inventory/IngredientSlot.IngredientSlot_C|Getindex (LocalVariables|GettmpSlot)))))
      (Transformation|SetWorldScale3D (Variables|/Game/Blueprints/Inventory/IngredientSlot.IngredientSlot_C|GetIngredientImage (LocalVariables|GettmpSlot)) "100.000000,100.000000,100.000000")
      (else
        (Rendering|Components|Sprite|SetSprite (Variables|/Game/Blueprints/Inventory/IngredientSlot.IngredientSlot_C|GetIngredientImage (LocalVariables|GettmpSlot)) "/Game/Sprites/OrthoWidth-144/ItemSlotPanel_Sprite.ItemSlotPanel_Sprite")
        (Transformation|SetWorldScale3D (Variables|/Game/Blueprints/Inventory/IngredientSlot.IngredientSlot_C|GetIngredientImage (LocalVariables|GettmpSlot)) "1.000000,1.000000,1.000000")))))

(fn SetIngredientCount
  (params (slot :type Ingredient%20Slot%20Object%20Reference))
  (LocalVariables|SettmpSlot slot)
  (if (>= (Variables|/Game/Blueprints/Inventory/IngredientSlot.IngredientSlot_C|Getindex (LocalVariables|GettmpSlot)) 9)
    (if (!= (Utilities|Array|Get(acopy) (Variables|/Game/Blueprints/GameSetting/GameSaveData.GameSaveData_C|GetingredientInfo (Variables|/Game/Blueprints/GameManager/GameManager.GameManager_C|GetgameSaveDataObject (Variables|Default|Getactor_GameManager))) (Variables|/Game/Blueprints/Inventory/IngredientSlot.IngredientSlot_C|Getindex (LocalVariables|GettmpSlot))) 0)
      (Rendering|Components|TextRender|SetText (Variables|/Game/Blueprints/Inventory/IngredientSlot.IngredientSlot_C|GetText (LocalVariables|GettmpSlot)) (Utilities|Text|ToText(String) (Utilities|String|Append "x" (Utilities|String|ToString(Integer) (Utilities|Array|Get(acopy) (Variables|/Game/Blueprints/GameSetting/GameSaveData.GameSaveData_C|GetingredientInfo (Variables|/Game/Blueprints/GameManager/GameManager.GameManager_C|GetgameSaveDataObject (Variables|Default|Getactor_GameManager))) (Variables|/Game/Blueprints/Inventory/IngredientSlot.IngredientSlot_C|Getindex (LocalVariables|GettmpSlot)))))) :!label _label)
      (else
        (Rendering|Components|TextRender|SetText (Variables|/Game/Blueprints/Inventory/IngredientSlot.IngredientSlot_C|GetText (LocalVariables|GettmpSlot)) (Utilities|Text|MakeLiteralText " "))))
    (else
      (goto _label))))

(fn ChecktheEnableArea
  (bind _returnvalue (Game|GetPlayerController 0))
  (bind _worldlocation (Game|Player|ConvertMouseLocationToWorldSpace _returnvalue))
  (bind (_x _y _z) (Math|Vector|BreakVector _worldlocation))
  (return (or (or (>= _x 1.2e+02) (<= _x -1.2e+02)) (or (>= _z 72.0) (<= _z -142.0)))))

(fn ChecktheCount
  (if (== (Utilities|Array|Get(acopy) (Variables|/Game/Blueprints/GameSetting/GameSaveData.GameSaveData_C|GetingredientInfo (Variables|/Game/Blueprints/GameManager/GameManager.GameManager_C|GetgameSaveDataObject (Variables|Default|Getactor_GameManager))) (Variables|Default|GetselectIndex)) 0)
    (Rendering|Components|TextRender|SetTextRenderColor (Variables|Default|GetText_Select) (Math|Color|MakeColor 0 0 255 255))
    (Collision|SetCollisionEnabled (Variables|Default|GetButton_Select) "NoCollision")
    (else
      (Rendering|Components|TextRender|SetTextRenderColor (Variables|Default|GetText_Select) (Math|Color|MakeColor 255 255 255 255))
      (Collision|SetCollisionEnabled (Variables|Default|GetButton_Select) "QueryAndPhysics"))))

(fn ResetSlotLocation
  (params (slot :type Ingredient%20Slot%20Object%20Reference) (index :type Integer))
  (LocalVariables|SetlocalIndex index)
  (LocalVariables|Setlocation_PositionX (+ (* (LocalVariables|GetlocalIndex) 36.0) -92.0))
  (Transformation|SetActorLocation slot (Math|Vector|MakeVector (LocalVariables|Getlocation_PositionX) 3.4e+02 -97.0) false true))