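; Guild ingredient store actor that stays hidden until ShowIngredientInventory reveals it and enables its slots.
; Stock is built from the guild rank table's low, mid and high material tiers, plus one special ingredient when IsRare is set.
; Slots show ingredient sprites with count/stock text.
; Touch and Tick drive horizontal drag-scrolling of the panel inside a bounded area, snapping back when X exceeds zero.
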(event EventBeginPlay
  ;[1 1 1] 초기화
  (Rendering|SetActorHiddenInGame true)
  (Collision|SetActorEnableCollision false))

(event EventActorOnInputTouchEnd
  (params (FingerIndex :type ETouchIndex%20Enum :default "Touch1"))
  (bind _returnvalue (Game|GetPlayerController 0))
  (bind (_locationx _locationy) (Game|Player|GetMousePosition _returnvalue))
  ;[1 1 1] 드래그 시작/종료
  (Variables|Default|SetisPressed false)
  (Variables|Default|SetisDragged false)
  (Variables|Default|Setvector_MousePosition (Math|Vector|MakeVector _locationx _locationy 26.0)))

(event EventActorOnInputTouchBegin
  (params (FingerIndex :type ETouchIndex%20Enum :default "Touch1"))
  (bind _returnvalue (Game|GetPlayerController 0))
  (bind (_locationx _locationy) (Game|Player|GetMousePosition _returnvalue))
  ;[1 1 1] 드래그 시작/종료
  (Variables|Default|SetisPressed true)
  (Variables|Default|Setvector_MousePosition (Math|Vector|MakeVector _locationx _locationy 26.0)))

(event EventShowIngredientInventory
  (params (SceneFrom :type Actor%20Object%20Reference))
  ;[1 1 1] 재료 상점 활성화
  (Variables|Default|Setactor_AttachToScene SceneFrom)
  (Rendering|SetActorHiddenInGame false)
  (Collision|SetActorEnableCollision true)
  (|아이템슬롯활셩화)
  (|배열초기화))

(event EventTick
  (params (DeltaSeconds :type Float%20%28single-precision%29))
  (bind _returnvalue (Game|GetPlayerController 0))
  (bind _locationx (Game|Player|GetMousePosition _returnvalue))
  (bind _returnvalue_2 (Math|Vector|MakeVector _locationx 0.0 26.0))
  ;[1 1 1] 드래그 이벤트
  (if (Variables|Default|GetisPressed) ; 클릭중인가
    (bind _disable (CallFunction|ChecktheEnableArea))
    (if _disable
      (Variables|Default|SetisPressed false)
      (elif (|드래그가되었는가체크_2) ; 드래그가 되었는가?
        (Variables|Default|SetisDragged true)
        (bind _ismovable (CallFunction|CheckthePosition))
        (if _ismovable ; 슬롯이 이동 가능한가?
          (Transformation|SetActorLocation (Variables|Default|Getactor_Panel) (|슬롯이동좌표계산) false false)
          (Variables|Default|Setvector_MousePosition _returnvalue_2)
          (else
            (Transformation|SetActorLocation (Variables|Default|Getactor_Panel) (|초기슬롯좌표계산) false false)
            (Variables|Default|Setvector_MousePosition _returnvalue_2)))))))

(fn ConstructionScript)

(fn SetSlot
  (params (slot :type Ingredient%20Slot%20Object%20Reference) (index :type Integer))
  (bind _array_ingredientstock (Variables|Default|Getarray_IngredientStock))
  (bind _item (Utilities|Array|Get(acopy) _array_ingredientstock index))
  (LocalVariables|Set_Slot slot)
  (if (< index 9)
    (Rendering|Components|Sprite|SetSprite (Variables|/Game/Blueprints/Inventory/IngredientSlot.IngredientSlot_C|GetIngredientImage (LocalVariables|Get_Slot)) (Utilities|Array|Get(acopy) (Variables|/Game/Blueprints/GameManager/GameManager.GameManager_C|Getarray_IngredientSprite (Variables|Default|Getactor_GameManager)) index))
    (Transformation|SetWorldScale3D (Variables|/Game/Blueprints/Inventory/IngredientSlot.IngredientSlot_C|GetIngredientImage (LocalVariables|Get_Slot)) "100.000000,100.000000,100.000000")
    (if (!= _item 0)
      (Rendering|Components|TextRender|SetText (Variables|/Game/Blueprints/Inventory/IngredientSlot.IngredientSlot_C|GetText (LocalVariables|Get_Slot)) (Utilities|Text|ToText(String) (Utilities|String|Append (Utilities|String|ToString(Integer) (Utilities|Array|Get(acopy) (Variables|Default|Getarray_IngredientCount) index)) "/" (Utilities|String|ToString(Integer) _item))))
      (else
        (Rendering|Components|TextRender|SetText (Variables|/Game/Blueprints/Inventory/IngredientSlot.IngredientSlot_C|GetText (LocalVariables|Get_Slot)) (Utilities|Text|MakeLiteralText "-"))))))

(fn ChecktheEnableArea
  (bind _returnvalue (Game|GetPlayerController 0))
  (bind _worldlocation (Game|Player|ConvertMouseLocationToWorldSpace _returnvalue))
  (bind (_x _y _z) (Math|Vector|BreakVector _worldlocation))
  (return (or (or (>= _x 1.2e+02) (<= _x -1.2e+02)) (or (>= _z 72.0) (<= _z -142.0)))))

(fn CheckthePosition
  (return (<= (.X (Math|Vector|BreakVector (Transformation|GetActorLocation (Variables|Default|Getactor_Panel)))) 0.0)))

(fn ChecktheRare
  (bind _returnvalue (Utilities|GetDataTableRow "/Game/Blueprints/GuildRankTable.GuildRankTable" (Utilities|String|StringToName (Utilities|String|ToString(Integer) (Variables|/Game/Blueprints/GameSetting/GameSaveData.GameSaveData_C|GetguildRank (Variables|/Game/Blueprints/GameManager/GameManager.GameManager_C|GetgameSaveDataObject (Variables|Default|Getactor_GameManager))))))
    (:then
      (if (>= (Math|Float|Truncate (* 100 (.레어소재확률 _returnvalue))) (Math|Random|RandomIntegerinRange 1 100)) ; 특수 재료
        (Variables|Default|SetisRare true)
        (else
          (Variables|Default|SetisRare false))))))