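; Guild main menu actor that routes touch input to the weapon store or back to the house scene.
; Buttons fire only when touch release lands on the component recorded at touch begin.
; The weapon store button disables collision, slides the guild menu actor along X with a timeline, then enables the weapon menu's collision.
; The house button clears sword-index and select-box arrays, then calls the game manager's home-scene message.
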(event `self.ReceiveBeginPlay`
  ;[1 1 1] 초기화
  (`self.SetActorEnableCollision` false))

(event `self.Button_WeaponStore.OnInputTouchEnd`
  (params (FingerIndex :type "ETouchIndex Enum" :default "Touch1") (TouchedComponent :type "PrimitiveComponent Object Reference"))
  ;[1 1 1] 무기 상점으로 이동
  (if (== TouchedComponent (`self.enableButton`))
    (`self.SetActorEnableCollision` false)
    (set `self.vector_OriginalLocation` (`self.K2_GetActorLocation` (`self.actor_GuildMenu`)))
    (bind (_direction `_인터페이스_이동`) (`Timeline|ToWeaponStore` :!via `PlayFromStart`)
      (:`Update`
        (`self.K2_SetActorLocation` (`self.actor_GuildMenu`) (+ (`KismetMathLibrary.MakeVector` (* `_인터페이스_이동` -288.0)) (`self.vector_OriginalLocation`)) false false))
      (:`Finished`
        (`self.SetActorEnableCollision` (`self.actor_WeaponMenu`) true)))))

(event `self.Button_WeaponStore.OnInputTouchBegin`
  (params (FingerIndex :type "ETouchIndex Enum" :default "Touch1") (TouchedComponent :type "PrimitiveComponent Object Reference"))
  ;[1 1 1] 무기 상점으로 이동
  (set `self.enableButton` TouchedComponent))

(event `self.Button_ToHouse.OnInputTouchEnd`
  (params (FingerIndex :type "ETouchIndex Enum" :default "Touch1") (TouchedComponent :type "PrimitiveComponent Object Reference"))
  ;[1 1 1] HouseMenu로 이동
  (if (== TouchedComponent (`self.enableButton`))
    (`KismetArrayLibrary.Array_Resize` (`self.openedSwordIndex`))
    (`KismetArrayLibrary.Array_Resize` (`self.selectBoxLocation`))
    (message `/Game/Blueprints/GameManager/GameManagerInterface.CallScene_Home` (`self.gameManager_Actor`))))

(event `self.Button_ToHouse.OnInputTouchBegin`
  (params (FingerIndex :type "ETouchIndex Enum" :default "Touch1") (TouchedComponent :type "PrimitiveComponent Object Reference"))
  ;[1 1 1] HouseMenu로 이동
  (set `self.enableButton` TouchedComponent))

(fn `UserConstructionScript`)