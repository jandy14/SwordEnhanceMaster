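; Guild weapon store actor: a hidden world-space touch menu that opens over a calling scene, disabling that scene's collision until closed.
; On open it fills slots from the save's unlocked swords; the slot panel drags horizontally via Tick.
; A selected sword shows SwordList table details, and tapping either side adjusts quantity within stock.
; Buy adds swords to the saved inventory, reduces stock and saves, with no currency check.
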(event OnInputTouchEnd(Button_Close)
  (params (FingerIndex :type ETouchIndex%20Enum :default "Touch1") (TouchedComponent :type Primitive%20Component%20Object%20Reference))
  ;[1 1 1] 인벤토리 닫기
  (if (== TouchedComponent (Variables|Default|GetEnableButton))
    (Collision|SetActorEnableCollision (Variables|Default|Getactor_AttachToScene) true)
    (Rendering|SetActorHiddenInGame true)
    (Collision|SetActorEnableCollision false)
    (|아이템슬롯비활셩화)
    (|배열해제)))

(event OnInputTouchBegin(Button_Close)
  (params (FingerIndex :type ETouchIndex%20Enum :default "Touch1") (TouchedComponent :type Primitive%20Component%20Object%20Reference))
  ;[1 1 1] 인벤토리 닫기
  (Variables|Default|SetEnableButton TouchedComponent))

(event OnInputTouchEnd(Button_Buy)
  (params (FingerIndex :type ETouchIndex%20Enum :default "Touch1") (TouchedComponent :type Primitive%20Component%20Object%20Reference))
  ;[1 1 1] 구입 버튼 이벤트
  (if (== TouchedComponent (Variables|Default|GetEnableButton))
    (for (_array_element _array_index) (Variables|Default|Getarray_SwordCount)
      (Variables|Default|SetloopIndex _array_index)
      (for _index (range 1 _array_element)
        (|아이템인벤토리에추가))
      (|재고량새로고침 _array_element)
      (CallFunction|RefreshSlotText _array_element))
    (SaveGame|SaveGametoSlot (Variables|/Game/Blueprints/GameManager/GameManager.GameManager_C|GetgameSaveDataObject (Variables|Default|Getactor_GameManager)) "GameSaveSlot1")))

(event OnInputTouchBegin(Button_Buy)
  (params (FingerIndex :type ETouchIndex%20Enum :default "Touch1") (TouchedComponent :type Primitive%20Component%20Object%20Reference))
  ;[1 1 1] 구입 버튼 이벤트
  (Variables|Default|SetEnableButton TouchedComponent))

(event OnInputTouchEnd(InfoArea)
  (params (FingerIndex :type ETouchIndex%20Enum :default "Touch1") (TouchedComponent :type Primitive%20Component%20Object%20Reference))
  ;[1 1 1] 수량 증감
  (if (== TouchedComponent (Variables|Default|GetEnableButton))
    (if (not (Variables|Default|GetisDragged))
      (if (Variables|Default|GetisSelected)
        (if (> (.X (Math|Vector|BreakVector (.WorldLocation (Game|Player|ConvertMouseLocationToWorldSpace (Game|GetPlayerController 0))))) 0.0)
          (|수량증가)
          (else
            (|수량감소)))
        (CallFunction|RefreshText)
        (CallFunction|RefreshSlotText (Variables|Default|GetselectedIndex))))))

(event OnInputTouchBegin(InfoArea)
  (params (FingerIndex :type ETouchIndex%20Enum :default "Touch1") (TouchedComponent :type Primitive%20Component%20Object%20Reference))
  ;[1 1 1] 수량 증감
  (Variables|Default|SetEnableButton TouchedComponent))

(event EventSelectItem
  (params (Index :type Integer))
  ;[1 1 1] Select Item 이벤트
  (if (< Index (Utilities|Array|Length (Variables|Default|Getarray_OpenedSwordIndex)))
    (|선택된아이템세팅 Index)
    (else
      (|선택창초기화))))

(event EventBeginPlay
  ;[1 1 1] 초기화
  (Collision|SetActorEnableCollision false)
  (Rendering|SetActorHiddenInGame true))

(event EventActorOnInputTouchEnd
  (params (FingerIndex :type ETouchIndex%20Enum :default "Touch1"))
  (bind _returnvalue (Game|GetPlayerController 0))
  (bind (_locationx _locationy) (Game|Player|GetMousePosition _returnvalue))
  ;[1 1 1] 드래그 시작/종료
  (Variables|Default|SetisPressed false)
  (Variables|Default|SetisDragged false)
  (Variables|Default|Setvector_MousePosition (Math|Vector|MakeVector _locationx _locationy 26.0)))

(event EventActorOnInputTouchBegin
  (params (FingerIndex :type ETouchIndex%20Enum :default "Touch1"))
  (bind _returnvalue (Game|GetPlayerController 0))
  (bind (_locationx _locationy) (Game|Player|GetMousePosition _returnvalue))
  ;[1 1 1] 드래그 시작/종료
  (Variables|Default|SetisPressed true)
  (Variables|Default|Setvector_MousePosition (Math|Vector|MakeVector _locationx _locationy 26.0)))

(event EventShowInventory
  (params (SceneFrom :type Actor%20Object%20Reference) (FromEnhancement :type Boolean) (FromWeaponStore :type Boolean))
  ;[1 1 1] 인벤토리 활성화
  (bind _output_get (Variables|Default|Setactor_AttachToScene SceneFrom))
  (Collision|SetActorEnableCollision _output_get false)
  (Rendering|SetActorHiddenInGame false)
  (Collision|SetActorEnableCollision true)
  (|아이템슬롯활셩화)
  (|배열초기화)
  (|아이템정보창초기화)
  (|아이템슬롯초기화))

(event EventTick
  (params (DeltaSeconds :type Float%20%28single-precision%29))
  (bind _returnvalue (Game|GetPlayerController 0))
  (bind _locationx (Game|Player|GetMousePosition _returnvalue))
  (bind _returnvalue_2 (Math|Vector|MakeVector _locationx 0.0 26.0))
  ;[1 1 1] 드래그 이벤트
  (if (Variables|Default|GetisPressed) ; 클릭중인가
    (bind _disable (CallFunction|ChecktheEnableArea))
    (if _disable
      (Variables|Default|SetisPressed false)
      (elif (|드래그가되었는가체크) ; 드래그가 되었는가?
        (Variables|/Game/Blueprints/Inventory/Slot.Slot_C|SetisSelectable (Variables|Default|Getactor_CurrentSlot) false)
        (Variables|Default|SetisDragged true)
        (bind _ismovable (CallFunction|CheckthePosition))
        (if _ismovable ; 슬롯이 이동 가능한가?
          (Transformation|SetActorLocation (Variables|Default|Getactor_Panel) (|슬롯이동좌표계산) false false)
          (Variables|Default|Setvector_MousePosition _returnvalue_2)
          (else
            (Transformation|SetActorLocation (Variables|Default|Getactor_Panel) (|초기슬롯좌표계산) false false)
            (Variables|Default|Setvector_MousePosition _returnvalue_2)))))))

(fn ConstructionScript)

(fn SetSlot
  (params (slot :type Slot%20Object%20Reference) (index :type Integer))
  (bind _swordimage (Variables|/Game/Blueprints/Inventory/Slot.Slot_C|GetSwordImage slot))
  (if (<= index (- (Utilities|Array|Length (Variables|Default|Getarray_OpenedSwordIndex)) 1))
    (Rendering|Components|Sprite|SetSprite _swordimage (Utilities|Array|Get(acopy) (Variables|/Game/Blueprints/GameManager/GameManager.GameManager_C|Getarray_SwordSprite (Variables|Default|Getactor_GameManager)) (Utilities|Array|Get(acopy) (Variables|Default|Getarray_OpenedSwordIndex) index)))
    (Transformation|SetWorldScale3D _swordimage "100.000000,100.000000,100.000000")
    (elif (< index 9)
      (Rendering|Components|TextRender|SetText (Variables|/Game/Blueprints/Inventory/Slot.Slot_C|GetText slot) (Utilities|Text|MakeLiteralText " ")))))

(fn ChecktheEnableArea
  (bind _returnvalue (Game|GetPlayerController 0))
  (bind _worldlocation (Game|Player|ConvertMouseLocationToWorldSpace _returnvalue))
  (bind (_x _y _z) (Math|Vector|BreakVector _worldlocation))
  (return (or (or (>= _x 1.2e+02) (<= _x -1.2e+02)) (or (>= _z 72.0) (<= _z -142.0)))))

(fn ResetSlotLocation
  (params (slot :type Slot%20Object%20Reference) (index :type Integer))
  (LocalVariables|SetlocalIndex index)
  (LocalVariables|Setlocation_PositionX (+ (* (LocalVariables|GetlocalIndex) 36.0) -92.0))
  (Transformation|SetActorLocation slot (Math|Vector|MakeVector (LocalVariables|Getlocation_PositionX) 7.4e+02 26.0) false true))

(fn CheckthePosition
  (return (<= (.X (Math|Vector|BreakVector (Transformation|GetActorLocation (Variables|Default|Getactor_Panel)))) 0.0)))

(fn RefreshText
  (Rendering|Components|TextRender|SetText (Variables|Default|GetText_Count) (Utilities|Text|ToText(String) (Utilities|String|Append "수량 : " (Utilities|String|ToString(Integer) (Utilities|Array|Get(acopy) (Variables|Default|Getarray_SwordCount) (Variables|Default|GetselectedIndex))) "/" (Utilities|String|ToString(Integer) (Utilities|Array|Get(acopy) (Variables|Default|Getarray_SwordStock) (Variables|Default|GetselectedIndex)))))))

(fn RefreshSlotText
  (params (index :type Integer))
  (LocalVariables|SetlocalIndex index)
  (if (and (>= (LocalVariables|GetlocalIndex) (Utilities|Array|Length (Variables|Default|Getarray_SwordCount))) (== (Utilities|Array|Get(acopy) (Variables|Default|Getarray_SwordCount) (LocalVariables|GetlocalIndex)) 0))
    (Rendering|Components|TextRender|SetText (Variables|/Game/Blueprints/Inventory/Slot.Slot_C|GetText (Utilities|Array|Get(acopy) (Variables|Default|Getarray_StoreSlot) (Math|Integer|%(Integer) (LocalVariables|GetlocalIndex) 8))) (Utilities|Text|MakeLiteralText "-"))
    (else
      (Rendering|Components|TextRender|SetText (Variables|/Game/Blueprints/Inventory/Slot.Slot_C|GetText (Utilities|Array|Get(acopy) (Variables|Default|Getarray_StoreSlot) (Math|Integer|%(Integer) (LocalVariables|GetlocalIndex) 8))) (Utilities|Text|ToText(String) (Utilities|String|Append "x" (Utilities|String|ToString(Integer) (Utilities|Array|Get(acopy) (Variables|Default|Getarray_SwordCount) (LocalVariables|GetlocalIndex)))))))))