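; Guild weapon menu actor with touch buttons that open the weapon store, open the inventory for selling, or slide back to the guild main screen via a timeline.
; It totals checked weapons' prices, looked up by enhancement count.
; Selling removes those weapons, adds money and reliability scaled by the guild rank DataTable, and spends reliability on rank-ups up to a cap.
; It then refreshes the user info bar and saves the game.
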(event `self.ReceiveBeginPlay`
  ;[1 1 1] 비활성화
  (`self.SetActorEnableCollision` false))

(event `self.Button_BuyWeapon.OnInputTouchEnd`
  (params (FingerIndex :type "ETouchIndex Enum" :default "Touch1") (TouchedComponent :type "PrimitiveComponent Object Reference"))
  ;[1 1 1] 무기 구입 버튼 이벤트
  (if (== TouchedComponent (`self.enableButton`))
    (message `/Game/Blueprints/Inventory/InventoryManager.ShowInventory` (`self.actor_WeaponStore`) self false false)))

(event `self.Button_BuyWeapon.OnInputTouchBegin`
  (params (FingerIndex :type "ETouchIndex Enum" :default "Touch1") (TouchedComponent :type "PrimitiveComponent Object Reference"))
  ;[1 1 1] 무기 구입 버튼 이벤트
  (set `self.enableButton` TouchedComponent))

(event `self.Button_SellWeapon.OnInputTouchEnd`
  (params (FingerIndex :type "ETouchIndex Enum" :default "Touch1") (TouchedComponent :type "PrimitiveComponent Object Reference"))
  ;[1 1 1] 무기 판매 버튼 이벤트
  (if (== TouchedComponent (`self.enableButton`))
    (message `/Game/Blueprints/Inventory/InventoryManager.ShowInventory` (`self.actor_WeaponInventory`) self false true)))

(event `self.Button_SellWeapon.OnInputTouchBegin`
  (params (FingerIndex :type "ETouchIndex Enum" :default "Touch1") (TouchedComponent :type "PrimitiveComponent Object Reference"))
  ;[1 1 1] 무기 판매 버튼 이벤트
  (set `self.enableButton` TouchedComponent))

(event `/Game/Blueprints/Inventory/InventoryManager.CalculateWeaponPrice`
  (params (index :type Integer) (isChecked :type Boolean))
  (bind (_swordname _swordnumber `_소재강화` `_예리함강화` `_무게감강화` `_속성강화`) (break `/Game/Blueprints/SwordInfo` (`KismetArrayLibrary.Array_Get` (`/Game/Blueprints/GameSetting/GameSaveData.swordInfo` (`/Game/Blueprints/GameManager/GameManager.gameSaveDataObject` (`self.gameManager_Actor`))) index)))
  (bind _item (`KismetArrayLibrary.Array_Get` (`/Game/Blueprints/GameManager/GameManager.array_WeaponPrice` (`self.gameManager_Actor`)) (+ (+ `_소재강화` `_예리함강화` `_무게감강화`) (`KismetMathLibrary.Conv_BoolToInt` (`KismetTextLibrary.NotEqual_TextText` `_속성강화` "null")))))
  ;[1 1 1] Calculate Weapon Price 이벤트
  (if isChecked
    (set `self.totalPrice` (+ _item (`self.totalPrice`)))
    (else
      (set `self.totalPrice` (- (`self.totalPrice`) _item)))))

(event `/Game/Blueprints/Inventory/InventoryManager.SellWeapons`
  (bind _returnvalue (`KismetArrayLibrary.Array_Find` (`/Game/Blueprints/Inventory/WeaponInventory.array_CheckedWeapon` (`self.actor_WeaponInventory`)) true))
  ;[1 1 1] Sell Weapons 이벤트
  (while (`KismetArrayLibrary.Array_Contains` (`/Game/Blueprints/Inventory/WeaponInventory.array_CheckedWeapon` (`self.actor_WeaponInventory`)) true)
    (`KismetArrayLibrary.Array_Remove` (`/Game/Blueprints/GameSetting/GameSaveData.swordInfo` (`/Game/Blueprints/GameManager/GameManager.gameSaveDataObject` (`self.gameManager_Actor`))) _returnvalue)
    (`KismetArrayLibrary.Array_Remove` (`/Game/Blueprints/Inventory/WeaponInventory.array_CheckedWeapon` (`self.actor_WeaponInventory`)) _returnvalue))
  (bind _returnvalue_2 (`|GetDataTableRow` "/Game/Blueprints/GuildRankTable.GuildRankTable" (`KismetStringLibrary.Conv_StringToName` (`KismetStringLibrary.Conv_IntToString` (`/Game/Blueprints/GameSetting/GameSaveData.guildRank` (`/Game/Blueprints/GameManager/GameManager.gameSaveDataObject` (`self.gameManager_Actor`))))))
    (:`then`
      (set `/Game/Blueprints/GameSetting/GameSaveData.money` (+ (`/Game/Blueprints/GameSetting/GameSaveData.money` (`/Game/Blueprints/GameManager/GameManager.gameSaveDataObject` (`self.gameManager_Actor`))) (`KismetMathLibrary.FTrunc` (* (`self.totalPrice`) (`.무기매입가격_14_AE05F3A041D58E4C8C75969EECCF95E8` (break `/Game/Blueprints/GuildRankStruck` _returnvalue_2))))) (`/Game/Blueprints/GameManager/GameManager.gameSaveDataObject` (`self.gameManager_Actor`)))
      (bind _returnvalue_3 (`|GetDataTableRow` "/Game/Blueprints/GuildRankTable.GuildRankTable" (`KismetStringLibrary.Conv_StringToName` (`KismetStringLibrary.Conv_IntToString` (`/Game/Blueprints/GameSetting/GameSaveData.guildRank` (`/Game/Blueprints/GameManager/GameManager.gameSaveDataObject` (`self.gameManager_Actor`))))))
        (:`then`
          (bind _output_get (set `self.totalReliability` (* (`self.totalPrice`) (`.획득신뢰도_16_7E5B68BE489B98F4F0175A9E22C1364C` (break `/Game/Blueprints/GuildRankStruck` _returnvalue_3)))))
          (set `/Game/Blueprints/GameSetting/GameSaveData.reliability` (+ (`/Game/Blueprints/GameSetting/GameSaveData.reliability` (`/Game/Blueprints/GameManager/GameManager.gameSaveDataObject` (`self.gameManager_Actor`))) _output_get) (`/Game/Blueprints/GameManager/GameManager.gameSaveDataObject` (`self.gameManager_Actor`)))
          (`self.CheckTheGuildRank`)
          (message `/Game/Blueprints/WindowManager.RefreshTextBar` (`self.actor_UserInfoBar`))
          (set `self.totalPrice` 0)
          (set `self.totalReliability` 0.0)
          (`GameplayStatics.SaveGameToSlot` (`/Game/Blueprints/GameManager/GameManager.gameSaveDataObject` (`self.gameManager_Actor`)) "GameSaveSlot1"))))))

(event `self.Button_ToMain.OnInputTouchEnd`
  (params (FingerIndex :type "ETouchIndex Enum" :default "Touch1") (TouchedComponent :type "PrimitiveComponent Object Reference"))
  ;[1 1 1] GuildMain으로 이동
  (if (== TouchedComponent (`self.enableButton`))
    (`self.SetActorEnableCollision` false)
    (set `self.vector_OriginalLocation` (`self.K2_GetActorLocation` (`self.actor_GuildMenu`)))
    (bind (_direction `_인터페이스_이동`) (`Timeline|타임라인_0` :!via `PlayFromStart`)
      (:`Update`
        (`self.K2_SetActorLocation` (`self.actor_GuildMenu`) (+ (`KismetMathLibrary.MakeVector` (* `_인터페이스_이동` 288.0)) (`self.vector_OriginalLocation`)) false false))
      (:`Finished`
        (`self.SetActorEnableCollision` (`self.actor_GuildMain`) true)))))

(event `self.Button_ToMain.OnInputTouchBegin`
  (params (FingerIndex :type "ETouchIndex Enum" :default "Touch1") (TouchedComponent :type "PrimitiveComponent Object Reference"))
  ;[1 1 1] GuildMain으로 이동
  (set `self.enableButton` TouchedComponent))

(fn `CheckTheGuildRank`
  (while (< (`/Game/Blueprints/GameSetting/GameSaveData.guildRank` (`/Game/Blueprints/GameManager/GameManager.gameSaveDataObject` (`self.gameManager_Actor`))) 30)
    (bind _returnvalue (`|GetDataTableRow` "/Game/Blueprints/GuildRankTable.GuildRankTable" (`KismetStringLibrary.Conv_StringToName` (`KismetStringLibrary.Conv_IntToString` (+ (`/Game/Blueprints/GameSetting/GameSaveData.guildRank` (`/Game/Blueprints/GameManager/GameManager.gameSaveDataObject` (`self.gameManager_Actor`))) 1))))
      (:`then`
        (if (<= (break `/Game/Blueprints/GuildRankStruck` _returnvalue) (`KismetMathLibrary.FTrunc` (`/Game/Blueprints/GameSetting/GameSaveData.reliability` (`/Game/Blueprints/GameManager/GameManager.gameSaveDataObject` (`self.gameManager_Actor`)))))
          (set `/Game/Blueprints/GameSetting/GameSaveData.reliability` (- (`/Game/Blueprints/GameSetting/GameSaveData.reliability` (`/Game/Blueprints/GameManager/GameManager.gameSaveDataObject` (`self.gameManager_Actor`))) (`KismetMathLibrary.Conv_IntToDouble` (break `/Game/Blueprints/GuildRankStruck` _returnvalue))) (`/Game/Blueprints/GameManager/GameManager.gameSaveDataObject` (`self.gameManager_Actor`)))
          (set `/Game/Blueprints/GameSetting/GameSaveData.guildRank` (+ (`/Game/Blueprints/GameSetting/GameSaveData.guildRank` (`/Game/Blueprints/GameManager/GameManager.gameSaveDataObject` (`self.gameManager_Actor`))) 1) (`/Game/Blueprints/GameManager/GameManager.gameSaveDataObject` (`self.gameManager_Actor`)))
          (else
            (return))))))
  (return))

(fn `UserConstructionScript`)