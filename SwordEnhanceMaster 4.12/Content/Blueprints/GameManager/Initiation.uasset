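; Game manager actor that sets the initial state of the game's inventory, window, menu and scene actors on BeginPlay.
; It hides inventories, popup windows, slots, menus and the user info bar with collision off; House Main, Laboratory and Enhancement only lose collision.
; It also hides the scene manager's Black plane, disables its collision, and creates a Transparency dynamic material instance for it, stored on that manager as MIDTransparency.
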(event `self.ReceiveBeginPlay`
  ;[1 1 1] 인벤토리 비활성화
  (`self.SetActorHiddenInGame` (`self.actor_IngredientInventory`) true)
  (`self.SetActorHiddenInGame` (`self.actor_WeaponInventory`) true)
  (`self.SetActorEnableCollision` (`self.actor_IngredientInventory`) false)
  (`self.SetActorEnableCollision` (`self.actor_WeaponInventory`) false)
  ;[1 1 1] Window 비활성화
  (`self.SetActorHiddenInGame` (`self.actor_OneButtonWindow`) true)
  (`self.SetActorHiddenInGame` (`self.actor_TwoButtonsWindow`) true)
  (`self.SetActorEnableCollision` (`self.actor_OneButtonWindow`) false)
  (`self.SetActorEnableCollision` (`self.actor_TwoButtonsWindow`) false)
  ;[1 1 1] Scene 비활성화
  (`self.SetActorEnableCollision` (`self.actor_HouseMenu`) false)
  (`self.SetActorEnableCollision` (`self.actor_GuildMenu`) false)
  (`self.SetActorEnableCollision` (`self.actor_UserInfoBar`) false)
  (`self.SetActorEnableCollision` (`self.actor_HouseMain`) false)
  (`self.SetActorEnableCollision` (`self.actor_Laboratory`) false)
  (`self.SetActorEnableCollision` (`self.actor_Enhancement`) false)
  (for _array_element (`self.actor_Slot`)
    (`self.SetActorHiddenInGame` _array_element true)
    (`self.SetActorEnableCollision` _array_element false))
  (for _array_element_2 (`self.actor_IngredientSlot`)
    (`self.SetActorHiddenInGame` _array_element_2 true)
    (`self.SetActorEnableCollision` _array_element_2 false))
  (`SceneComponent.SetHiddenInGame` (`/Game/Blueprints/HouseMenu/HouseMenu.Scene` (`self.actor_HouseMenu`)) true true)
  (`self.SetActorHiddenInGame` (`self.actor_GuildMenu`) true)
  (`self.SetActorHiddenInGame` (`self.actor_UserInfoBar`) true)
  ;[1 1 1] 검은 판 비활성화
  (`SceneComponent.SetHiddenInGame` (`/Game/Blueprints/GameManager/SceneManager.Black` (`self.actor_SceneManager`)) true false)
  (`PrimitiveComponent.SetCollisionEnabled` (`/Game/Blueprints/GameManager/SceneManager.Black` (`self.actor_SceneManager`)) "NoCollision")
  ;[1 1 1] Material Instance 세팅
  (bind _returnvalue (`PrimitiveComponent.CreateDynamicMaterialInstance` (`/Game/Blueprints/GameManager/SceneManager.Black` (`self.actor_SceneManager`)) 0 "/Game/Materials/Transparency.Transparency"))
  (set `/Game/Blueprints/GameManager/SceneManager.MID_Transparency` _returnvalue (`self.actor_SceneManager`)))

(fn `UserConstructionScript`)