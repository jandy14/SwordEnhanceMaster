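; Camera manager actor that makes itself the player's view target when play begins.
; On BeginPlay it enables input on the referenced current-scene actor for player controller 0, then switches that controller's view to itself.
; It also prints the viewport width and height, apparently as debug output.
; Tick, overlap and construction logic are empty.
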(event `self.ReceiveBeginPlay`
  (bind (_returnvalue_x _returnvalue_y) (`KismetMathLibrary.BreakVector2D` (`WidgetLayoutLibrary.GetViewportSize`)))
  (`self.EnableInput` (`self.actor_CurrentScene`) (`GameplayStatics.GetPlayerController` 0))
  (`PlayerController.SetViewTargetWithBlend` (`GameplayStatics.GetPlayerController` 0) self 0.0 "VTBlend_Linear" 0.0 false)
  (`KismetSystemLibrary.PrintString` (`KismetStringLibrary.Conv_DoubleToString` _returnvalue_x))
  (`KismetSystemLibrary.PrintString` (`KismetStringLibrary.Conv_DoubleToString` _returnvalue_y)))

(fn `UserConstructionScript`)