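; Scene manager actor that switches the game between the main, house and guild menus behind a black fade.
; Each call event shows a collidable Black overlay and plays a timeline that drives its material's Amount parameter, swapping scene visibility when alpha reaches one.
; On finish, it hides the overlay, moves collision to the new scene and records it as current.
; House and guild transitions also refresh or reset related UI state.
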(event `/Game/Blueprints/GameManager/GameManagerInterface.CallScene_Home`
  ;[1 1 1] HouseMenu Scene 호출
  (`self.SetActorEnableCollision` (`self.actor_HouseMenu`) false)
  (`self.SetActorEnableCollision` (`self.actor_Laboratory`) false)
  (`self.SetActorEnableCollision` (`self.actor_Enhancement`) false)
  (`self.SetActorEnableCollision` (`self.actor_HouseMain`) false)
  (`SceneComponent.SetHiddenInGame` (`self.Black`) false false)
  (`PrimitiveComponent.SetCollisionEnabled` (`self.Black`) "QueryAndPhysics")
  (bind (_direction _alpha) (`Timeline|ToHouseMenu` :!via `PlayFromStart`)
    (:`Update`
      (`MaterialInstanceDynamic.SetScalarParameterValue` (`self.MID_Transparency`) "Amount" _alpha)
      (if (>= _alpha 1.0)
        (`self.SetActorHiddenInGame` (`self.actor_UserInfoBar`) false)
        (`self.SetActorHiddenInGame` (`self.actor_MainMenu`) true)
        (`SceneComponent.SetHiddenInGame` (`/Game/Blueprints/House/HouseMenu.Scene` (`self.actor_HouseMenu`)) false true)
        (`SceneComponent.SetHiddenInGame` (`/Game/Blueprints/Guild/GuildMenu.Scene` (`self.actor_GuildMenu`)) true true)
        (message `/Game/Blueprints/WindowManager.RefreshTextBar` (`self.actor_UserInfoBar`))))
    (:`Finished`
      (`SceneComponent.SetHiddenInGame` (`self.Black`) true false)
      (`PrimitiveComponent.SetCollisionEnabled` (`self.Black`) "NoCollision")
      (`self.SetActorEnableCollision` (`self.actor_CurrentScene`) false)
      (`self.SetActorEnableCollision` (`self.actor_HouseMenu`) true)
      (`self.SetActorEnableCollision` (`self.actor_HouseMain`) true)
      (set `self.actor_CurrentScene` (`self.actor_HouseMenu`))
      (set `/Game/Blueprints/Inventory/IngredientInventory.ingredientType` 0 (`self.actor_IngredientInventory`)))))

(event `/Game/Blueprints/GameManager/GameManagerInterface.CallScene_Guild`
  ;[1 1 1] GuildMenu Scene 호출
  (`self.SetActorEnableCollision` (`self.actor_GuildMenu`) false)
  (`self.SetActorEnableCollision` (`self.actor_GuildMain`) false)
  (`self.SetActorEnableCollision` (`self.actor_HouseMenu`) false)
  (`self.SetActorEnableCollision` (`self.actor_Laboratory`) false)
  (`self.SetActorEnableCollision` (`self.actor_Enhancement`) false)
  (`self.SetActorEnableCollision` (`self.actor_HouseMain`) false)
  (`SceneComponent.SetHiddenInGame` (`self.Black`) false false)
  (`PrimitiveComponent.SetCollisionEnabled` (`self.Black`) "QueryAndPhysics")
  (bind (_direction _alpha) (`Timeline|ToGuildMenu` :!via `PlayFromStart`) ; 씬 전환
    (:`Update`
      (`MaterialInstanceDynamic.SetScalarParameterValue` (`self.MID_Transparency`) "Amount" _alpha)
      (if (>= _alpha 1.0)
        (`SceneComponent.SetHiddenInGame` (`/Game/Blueprints/House/HouseMenu.Scene` (`self.actor_HouseMenu`)) true true)
        (`SceneComponent.SetHiddenInGame` (`/Game/Blueprints/Guild/GuildMenu.Scene` (`self.actor_GuildMenu`)) false true)))
    (:`Finished`
      (`SceneComponent.SetHiddenInGame` (`self.Black`) true false)
      (`PrimitiveComponent.SetCollisionEnabled` (`self.Black`) "NoCollision")
      (`self.SetActorEnableCollision` (`self.actor_CurrentScene`) false)
      (set `self.actor_CurrentScene` (`self.actor_GuildMenu`))
      (`self.SetActorEnableCollision` (`self.actor_GuildMenu`) true)
      (`self.SetActorEnableCollision` (`self.actor_GuildMain`) true)
      (message `/Game/Blueprints/GameManager/GameManagerInterface.Init_GuildMenu` (`self.actor_GuildMenu`)))))

(event `/Game/Blueprints/GameManager/GameManagerInterface.CallScene_Main`
  ;[1 1 1] MainMenu Scene 호출
  (`SceneComponent.SetHiddenInGame` (`self.Black`) false false)
  (`PrimitiveComponent.SetCollisionEnabled` (`self.Black`) "QueryAndPhysics")
  (bind (_direction _alpha) (`Timeline|ToMainMenu` :!via `PlayFromStart`) ; 씬 전환
    (:`Update`
      (`MaterialInstanceDynamic.SetScalarParameterValue` (`self.MID_Transparency`) "Amount" _alpha)
      (if (>= _alpha 1.0)
        (`self.SetActorHiddenInGame` (`self.actor_CurrentScene`) true)
        (`self.SetActorHiddenInGame` (`self.actor_UserInfoBar`) true)
        (`self.SetActorHiddenInGame` (`self.actor_MainMenu`) false)))
    (:`Finished`
      (`SceneComponent.SetHiddenInGame` (`self.Black`) true false)
      (`PrimitiveComponent.SetCollisionEnabled` (`self.Black`) "NoCollision")
      (`self.SetActorEnableCollision` (`self.actor_CurrentScene`) false)
      (`self.SetActorEnableCollision` (`self.actor_MainMenu`) true)
      (set `self.actor_CurrentScene` (`self.actor_MainMenu`)))))

(fn `UserConstructionScript`)