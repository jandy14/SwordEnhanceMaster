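; Game manager Blueprint that loads the guild save slot at start and handles the Android back button.
; SetTextBar writes rank and reliability to the user info bar, with gold fixed at zero, even without a save.
; Back opens a two-button quit prompt answered through SendButtonEvent: true shows a mocking refusal, false quits.
; CreateSaveFile writes a new save; CallSceneTestPage is empty, and scene-fade and UI-hiding logic is disconnected.
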(event `/Game/Blueprints/WindowManager.SendButtonEvent`
  (params (Answer :type Boolean))
  (`self.SetActorEnableCollision` (`self.actor_CurrentScene`) true)
  (switch `/Game/Blueprints/ActionList` (`self.actionList`)
    (:`NewEnumerator2`
      (if Answer
        (message `/Game/Blueprints/WindowManager.CallOneButtonWindow` (`self.actor_OneButtonWindow`) "싫은데?ㅋㅋㅋㅋㅋㅋ<br>ㅋㅋㅋㅋㅋㅋㅋㅋㅋㅋ<br>ㅋㅋㅋㅋㅋㅋㅋㅋㅋㅋ" (`self.actor_CurrentScene`))
        (else
          (`KismetSystemLibrary.QuitGame` (`GameplayStatics.GetPlayerController` 0) "Quit"))))))

(event `Key|Android_Back`
  (params (Key :type "Key Structure" :default "AnyKey"))
  (:`Pressed`
    (`self.SetActorEnableCollision` (`self.actor_CurrentScene`) false)
    (set `self.actionList` "NewEnumerator2")
    (message `/Game/Blueprints/WindowManager.CallWindow` (`self.actor_TwoButtonsWindow`) "종료하시겠습니까?" self)))

(event `self.ReceiveBeginPlay`
  ;[1 1 1] 세이브 데이터 로드
  (bind _returnvalue (`GameplayStatics.DoesSaveGameExist` "GameSaveSlot1"))
  (if _returnvalue
    (bind _returnvalue_2 (`GameplayStatics.LoadGameFromSlot` "GameSaveSlot1"))
    (bind _asgame_save_data (cast `/Game/Blueprints/GameSetting/GameSaveData` _returnvalue_2))
    (set `self.gameSaveDataObject` _asgame_save_data))
  (`self.SetTextBar`))

(event `/Game/Blueprints/GameManager/GameManagerInterface.CreateSaveFile`
  ;[1 1 1] 세이브 파일 생성
  (bind _returnvalue (`GameplayStatics.CreateSaveGameObject` "/Game/Blueprints/GameSetting/GameSaveData.GameSaveData_C"))
  (bind _asgame_save_data (cast `/Game/Blueprints/GameSetting/GameSaveData` _returnvalue))
  (bind _output_get (set `self.GameSaveDataObject` _asgame_save_data))
  (`GameplayStatics.SaveGameToSlot` _output_get "GameSaveSlot1"))

(event `/Game/Blueprints/GameManager/GameManagerInterface.CallScene_TestPage`
  ;[1 1 1] TestPage Scene 호출
)

(event `SetTextBar`
  ;[1 1 1] Set Text Bar 이벤트
  (`TextRenderComponent.K2_SetText` (`/Game/Blueprints/TextBar.GuildRank_Text` (`self.actor_UserInfoBar`)) (`KismetTextLibrary.Conv_StringToText` (`KismetStringLibrary.Concat_StrStr` "Rank : " (`KismetStringLibrary.Conv_IntToString` (`/Game/Blueprints/GameSetting/GameSaveData.guildRank` (`self.gameSaveDataObject`))))))
  (`TextRenderComponent.K2_SetText` (`/Game/Blueprints/TextBar.GuildReliability_Text` (`self.actor_UserInfoBar`)) (`KismetTextLibrary.Conv_StringToText` (`KismetStringLibrary.Concat_StrStr` "Exp : " (`KismetStringLibrary.Conv_IntToString` (`KismetMathLibrary.FTrunc` (`/Game/Blueprints/GameSetting/GameSaveData.reliability` (`self.gameSaveDataObject`)))))))
  (`TextRenderComponent.K2_SetText` (`/Game/Blueprints/TextBar.GuildMoney_Text` (`self.actor_UserInfoBar`)) (`KismetTextLibrary.Conv_StringToText` (`KismetStringLibrary.Concat_StrStr` "Gold : " (`KismetStringLibrary.Conv_IntToString` (`KismetMathLibrary.FTrunc` 0.0)) " G"))))

(fn `UserConstructionScript`)