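; Touch-driven ingredient inventory window actor that shows counts and sprites from GameManager in nine slots, with Normal and Rare tabs.
; The tab index times nine offsets into the GameManager arrays, and buttons act only when touch end matches the component stored on touch begin.
; Picking a slot updates the HouseMenu image, hides the window and messages the ingredient index to the opening scene.
; Visibility and collision toggles hand input between window, HouseMenu and current scene.
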(event `self.ReceiveBeginPlay`
  ;[1 1 1] 초기 설정
  (set `self.itemCount` (`|MakeArray` (`self.ItemCount1`) (`self.ItemCount2`) (`self.ItemCount3`) (`self.ItemCount4`) (`self.ItemCount5`) (`self.ItemCount6`) (`self.ItemCount7`) (`self.ItemCount8`) (`self.ItemCount9`)))
  (set `self.imageArray` (`|MakeArray` (`self.ImageSlot1`) (`self.ImageSlot2`) (`self.ImageSlot3`) (`self.ImageSlot4`) (`self.ImageSlot5`) (`self.ImageSlot6`) (`self.ImageSlot7`) (`self.ImageSlot8`) (`self.ImageSlot9`))))

(event `self.NormalButton.OnInputTouchEnd`
  (params (FingerIndex :type "ETouchIndex Enum" :default "Touch1") (TouchedComponent :type "PrimitiveComponent Object Reference"))
  ;[1 1 1] 일반 재료 버튼 이벤트
  (if (== TouchedComponent (`self.enableButton`))
    (bind _output_get (set `self.ingredientType` 0))
    (`self.SetIngredientItemSlot` _output_get)))

(event `self.NormalButton.OnInputTouchBegin`
  (params (FingerIndex :type "ETouchIndex Enum" :default "Touch1") (TouchedComponent :type "PrimitiveComponent Object Reference"))
  ;[1 1 1] 일반 재료 버튼 이벤트
  (set `self.enableButton` TouchedComponent))

(event `self.RareButton.OnInputTouchEnd`
  (params (FingerIndex :type "ETouchIndex Enum" :default "Touch1") (TouchedComponent :type "PrimitiveComponent Object Reference"))
  ;[1 1 1] 특수 재료 버튼 이벤트
  (if (== TouchedComponent (`self.enableButton`))
    (bind _output_get (set `self.ingredientType` 1))
    (`self.SetIngredientItemSlot` _output_get)))

(event `self.RareButton.OnInputTouchBegin`
  (params (FingerIndex :type "ETouchIndex Enum" :default "Touch1") (TouchedComponent :type "PrimitiveComponent Object Reference"))
  ;[1 1 1] 특수 재료 버튼 이벤트
  (set `self.enableButton` TouchedComponent))

(event `self.CloseButton_Sprite.OnInputTouchEnd`
  (params (FingerIndex :type "ETouchIndex Enum" :default "Touch1") (TouchedComponent :type "PrimitiveComponent Object Reference"))
  ;[1 1 1] 창 닫기
  (if (== TouchedComponent (`self.enableButton`))
    (`self.CloseInventory`)))

(event `self.CloseButton_Sprite.OnInputTouchBegin`
  (params (FingerIndex :type "ETouchIndex Enum" :default "Touch1") (TouchedComponent :type "PrimitiveComponent Object Reference"))
  ;[1 1 1] 창 닫기
  (set `self.enableButton` TouchedComponent))

(event `/Game/Blueprints/InventoryManager.SetIngredientItemSlot`
  (params (Index :type Integer))
  (bind _returnvalue (* Index 9))
  ;[1 1 1] 아이템 개수 세팅
  (for _index (range _returnvalue (+ (+ _returnvalue 8) 1))
    (bind _returnvalue_2 (mod _index 9))
    (`TextRenderComponent.K2_SetText` (`KismetArrayLibrary.Array_Get` (`self.itemCount`) _returnvalue_2) (`KismetTextLibrary.Conv_StringToText` (`KismetStringLibrary.Concat_StrStr` "x" (`KismetStringLibrary.Conv_IntToString` (`KismetArrayLibrary.Array_Get` (`/Game/Blueprints/GameManager.ingredientInfo` (`self.gameManager`)) _index)))))
    (bind _item (`KismetArrayLibrary.Array_Get` (`self.imageArray`) _returnvalue_2))
    ;[1 1 1] 아이템 이미지 세팅
    (`PaperSpriteComponent.SetSprite` _item (`KismetArrayLibrary.Array_Get` (`/Game/Blueprints/GameManager.ingredient_Sprite` (`self.gameManager`)) _index))
    (`SceneComponent.SetWorldScale3D` _item (0.4 0.1 0.4))))

(event `self.ColliderSlot1.OnInputTouchEnd`
  (params (FingerIndex :type "ETouchIndex Enum" :default "Touch1") (TouchedComponent :type "PrimitiveComponent Object Reference"))
  ;[1 1 1] 재료 선택
  (set `self.slotIndex` 0)
  (if (or (== TouchedComponent (`self.enableButton`)) (== (stale `self.ColliderSlot2.OnInputTouchEnd` TouchedComponent) (`self.enableButton`)) (== (stale `self.ColliderSlot3.OnInputTouchEnd` TouchedComponent) (`self.enableButton`)) (== (stale `self.ColliderSlot4.OnInputTouchEnd` TouchedComponent) (`self.enableButton`)) (== (stale `self.ColliderSlot5.OnInputTouchEnd` TouchedComponent) (`self.enableButton`)) (== (stale `self.ColliderSlot6.OnInputTouchEnd` TouchedComponent) (`self.enableButton`)) (== (stale `self.ColliderSlot7.OnInputTouchEnd` TouchedComponent) (`self.enableButton`)) (== (stale `self.ColliderSlot8.OnInputTouchEnd` TouchedComponent) (`self.enableButton`)) (== (stale `self.ColliderSlot9.OnInputTouchEnd` TouchedComponent) (`self.enableButton`))) :!label _label
    (message `/Game/Blueprints/InventoryManager.SelectIngredientItem` self (`self.slotIndex`))))

(event `/Game/Blueprints/InventoryManager.SelectIngredientItem`
  (params (Index :type Integer))
  (bind _ingredientimage (`/Game/Blueprints/HouseMenu.IngredientImage` (`self.houseMenu`)))
  (bind _returnvalue (+ Index (* (`self.ingredientType`) 9)))
  ;[1 1 1] 사용할 소재 선택
  (`PaperSpriteComponent.SetSprite` _ingredientimage (`KismetArrayLibrary.Array_Get` (`/Game/Blueprints/GameManager.ingredient_Sprite` (`self.gameManager`)) _returnvalue))
  (`SceneComponent.SetWorldScale3D` _ingredientimage (0.4 0.4 0.4))
  (`self.SetActorHiddenInGame` true)
  (`self.SetActorEnableCollision` false)
  (`self.SetActorEnableCollision` (`self.houseMenu`) true)
  (message `/Game/Blueprints/InventoryManager.SelectIngredient` (`self.attachToScene`) _returnvalue))

(event `self.ColliderSlot2.OnInputTouchEnd`
  (params (FingerIndex :type "ETouchIndex Enum" :default "Touch1") (TouchedComponent :type "PrimitiveComponent Object Reference"))
  ;[1 1 1] 재료 선택
  (set `self.slotIndex` 1)
  (goto _label))

(event `self.ColliderSlot1.OnInputTouchBegin`
  (params (FingerIndex :type "ETouchIndex Enum" :default "Touch1") (TouchedComponent :type "PrimitiveComponent Object Reference"))
  ;[1 1 1] 재료 선택
  (set `self.enableButton` TouchedComponent))

(event `self.ColliderSlot3.OnInputTouchEnd`
  (params (FingerIndex :type "ETouchIndex Enum" :default "Touch1") (TouchedComponent :type "PrimitiveComponent Object Reference"))
  ;[1 1 1] 재료 선택
  (set `self.slotIndex` 2)
  (goto _label))

(event `self.ColliderSlot2.OnInputTouchBegin`
  (params (FingerIndex :type "ETouchIndex Enum" :default "Touch1") (TouchedComponent :type "PrimitiveComponent Object Reference"))
  ;[1 1 1] 재료 선택
  (set `self.enableButton` TouchedComponent))

(event `self.ColliderSlot3.OnInputTouchBegin`
  (params (FingerIndex :type "ETouchIndex Enum" :default "Touch1") (TouchedComponent :type "PrimitiveComponent Object Reference"))
  ;[1 1 1] 재료 선택
  (set `self.enableButton` TouchedComponent))

(event `self.ColliderSlot4.OnInputTouchEnd`
  (params (FingerIndex :type "ETouchIndex Enum" :default "Touch1") (TouchedComponent :type "PrimitiveComponent Object Reference"))
  ;[1 1 1] 재료 선택
  (set `self.slotIndex` 3)
  (goto _label))

(event `self.ColliderSlot4.OnInputTouchBegin`
  (params (FingerIndex :type "ETouchIndex Enum" :default "Touch1") (TouchedComponent :type "PrimitiveComponent Object Reference"))
  ;[1 1 1] 재료 선택
  (set `self.enableButton` TouchedComponent))

(event `self.ColliderSlot5.OnInputTouchEnd`
  (params (FingerIndex :type "ETouchIndex Enum" :default "Touch1") (TouchedComponent :type "PrimitiveComponent Object Reference"))
  ;[1 1 1] 재료 선택
  (set `self.slotIndex` 4)
  (goto _label))

(event `self.ColliderSlot5.OnInputTouchBegin`
  (params (FingerIndex :type "ETouchIndex Enum" :default "Touch1") (TouchedComponent :type "PrimitiveComponent Object Reference"))
  ;[1 1 1] 재료 선택
  (set `self.enableButton` TouchedComponent))

(event `self.ColliderSlot6.OnInputTouchBegin`
  (params (FingerIndex :type "ETouchIndex Enum" :default "Touch1") (TouchedComponent :type "PrimitiveComponent Object Reference"))
  ;[1 1 1] 재료 선택
  (set `self.enableButton` TouchedComponent))

(event `self.ColliderSlot6.OnInputTouchEnd`
  (params (FingerIndex :type "ETouchIndex Enum" :default "Touch1") (TouchedComponent :type "PrimitiveComponent Object Reference"))
  ;[1 1 1] 재료 선택
  (set `self.slotIndex` 5)
  (goto _label))

(event `self.ColliderSlot7.OnInputTouchBegin`
  (params (FingerIndex :type "ETouchIndex Enum" :default "Touch1") (TouchedComponent :type "PrimitiveComponent Object Reference"))
  ;[1 1 1] 재료 선택
  (set `self.enableButton` TouchedComponent))

(event `self.ColliderSlot8.OnInputTouchBegin`
  (params (FingerIndex :type "ETouchIndex Enum" :default "Touch1") (TouchedComponent :type "PrimitiveComponent Object Reference"))
  ;[1 1 1] 재료 선택
  (set `self.enableButton` TouchedComponent))

(event `self.ColliderSlot7.OnInputTouchEnd`
  (params (FingerIndex :type "ETouchIndex Enum" :default "Touch1") (TouchedComponent :type "PrimitiveComponent Object Reference"))
  ;[1 1 1] 재료 선택
  (set `self.slotIndex` 6)
  (goto _label))

(event `self.ColliderSlot9.OnInputTouchBegin`
  (params (FingerIndex :type "ETouchIndex Enum" :default "Touch1") (TouchedComponent :type "PrimitiveComponent Object Reference"))
  ;[1 1 1] 재료 선택
  (set `self.enableButton` TouchedComponent))

(event `self.ColliderSlot8.OnInputTouchEnd`
  (params (FingerIndex :type "ETouchIndex Enum" :default "Touch1") (TouchedComponent :type "PrimitiveComponent Object Reference"))
  ;[1 1 1] 재료 선택
  (set `self.slotIndex` 7)
  (goto _label))

(event `self.ColliderSlot9.OnInputTouchEnd`
  (params (FingerIndex :type "ETouchIndex Enum" :default "Touch1") (TouchedComponent :type "PrimitiveComponent Object Reference"))
  ;[1 1 1] 재료 선택
  (set `self.slotIndex` 8)
  (goto _label))

(event `/Game/Blueprints/InventoryManager.ShowIngredientInventory`
  (params (SceneFrom :type "Actor Object Reference"))
  ;[1 1 1] 재료창 활성화
  (set `self.attachToScene` SceneFrom)
  (`self.SetActorEnableCollision` (`self.houseMenu`) false)
  (`self.SetActorHiddenInGame` false)
  (`self.SetActorEnableCollision` true)
  (message `/Game/Blueprints/InventoryManager.SetIngredientItemSlot` self (`self.ingredientType`)))

(event `CloseInventory`
  ;[1 1 1] 인벤토리 닫기
  (`self.SetActorHiddenInGame` true)
  (`self.SetActorEnableCollision` false)
  (`self.SetActorEnableCollision` (`/Game/Blueprints/GameManager.currentScene` (`self.gameManager`)) true))

(fn `UserConstructionScript`)