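; Test page actor for trying out dynamic force feedback (vibration) through touch buttons, with a button back to the main menu via GameManager.
; Step buttons adjust intensity and duration, and sprite toggles pick the left/right large and small motors.
; These values feed one dynamic force feedback node with start, update and stop, whose completion opens a popup.
; Each button acts on touch end only if it matches the component stored on touch begin.
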(event `self.ReceiveBeginPlay`)

(event `self.ReceiveActorBeginOverlap`
  (params (OtherActor :type "Actor Object Reference")))

(event `self.ReceiveTick`
  (params (DeltaSeconds :type "Float (single-precision)")))

(event `self.Vibration_Button.OnInputTouchBegin`
  (params (FingerIndex :type "ETouchIndex Enum" :default "Touch1") (TouchedComponent :type "PrimitiveComponent Object Reference"))
  ;[1 1 1] 진동
  (set `self.current_Button` TouchedComponent))

(event `self.Vibration_Button.OnInputTouchEnd`
  (params (FingerIndex :type "ETouchIndex Enum" :default "Touch1") (TouchedComponent :type "PrimitiveComponent Object Reference"))
  ;[1 1 1] 진동
  (if (== TouchedComponent (`self.current_Button`))
    (`PlayerController.PlayDynamicForceFeedback` (`GameplayStatics.GetPlayerController` 0) (`self.intensity`) (`self.time`) (`self.leftLarge`) (`self.leftSmall`) (`self.rightLarge`) (`self.rightSmall`) :!label _label)
    (message `/Game/Blueprints/WindowManager.CallOneButtonWindow` (`self.oneButtonWindow`) "진동 끝!" self)))

(event `self.VibrationUpdate_Button.OnInputTouchBegin`
  (params (FingerIndex :type "ETouchIndex Enum" :default "Touch1") (TouchedComponent :type "PrimitiveComponent Object Reference"))
  ;[1 1 1] 진동
  (set `self.current_Button` TouchedComponent))

(event `self.VibrationStop_Button.OnInputTouchBegin`
  (params (FingerIndex :type "ETouchIndex Enum" :default "Touch1") (TouchedComponent :type "PrimitiveComponent Object Reference"))
  ;[1 1 1] 진동
  (set `self.current_Button` TouchedComponent))

(event `self.VibrationStop_Button.OnInputTouchEnd`
  (params (FingerIndex :type "ETouchIndex Enum" :default "Touch1") (TouchedComponent :type "PrimitiveComponent Object Reference"))
  ;[1 1 1] 진동
  (if (== TouchedComponent (`self.current_Button`))
    (goto _label :!via `Stop`)))

(event `self.VibrationUpdate_Button.OnInputTouchEnd`
  (params (FingerIndex :type "ETouchIndex Enum" :default "Touch1") (TouchedComponent :type "PrimitiveComponent Object Reference"))
  ;[1 1 1] 진동
  (if (== TouchedComponent (`self.current_Button`))
    (goto _label :!via `Update`)))

(event `self.VibrationPowerDown.OnInputTouchEnd`
  (params (FingerIndex :type "ETouchIndex Enum" :default "Touch1") (TouchedComponent :type "PrimitiveComponent Object Reference"))
  ;[1 1 1] 진동 세기 조절
  (if (== TouchedComponent (`self.current_Button`))
    (bind _output_get (set `self.intensity` (- (`self.intensity`) 0.1)))
    (`TextRenderComponent.K2_SetText` (`self.VibrationPower_Text`) (`KismetTextLibrary.Conv_DoubleToText` _output_get "HalfToEven"))))

(event `self.VibrationPowerDown.OnInputTouchBegin`
  (params (FingerIndex :type "ETouchIndex Enum" :default "Touch1") (TouchedComponent :type "PrimitiveComponent Object Reference"))
  ;[1 1 1] 진동 세기 조절
  (set `self.current_Button` TouchedComponent))

(event `self.VibrationPowerUp.OnInputTouchEnd`
  (params (FingerIndex :type "ETouchIndex Enum" :default "Touch1") (TouchedComponent :type "PrimitiveComponent Object Reference"))
  ;[1 1 1] 진동 세기 조절
  (if (== TouchedComponent (`self.current_Button`))
    (bind _output_get (set `self.intensity` (+ (`self.intensity`) 0.1)))
    (`TextRenderComponent.K2_SetText` (`self.VibrationPower_Text`) (`KismetTextLibrary.Conv_DoubleToText` _output_get "HalfToEven"))))

(event `self.VibrationPowerUp.OnInputTouchBegin`
  (params (FingerIndex :type "ETouchIndex Enum" :default "Touch1") (TouchedComponent :type "PrimitiveComponent Object Reference"))
  ;[1 1 1] 진동 세기 조절
  (set `self.current_Button` TouchedComponent))

(event `self.TimeUp.OnInputTouchEnd`
  (params (FingerIndex :type "ETouchIndex Enum" :default "Touch1") (TouchedComponent :type "PrimitiveComponent Object Reference"))
  ;[1 1 1] 진동 시간 조절
  (if (== TouchedComponent (`self.current_Button`))
    (bind _output_get (set `self.time` (+ (`self.time`) 0.1)))
    (`TextRenderComponent.K2_SetText` (`self.Time_Text`) (`KismetTextLibrary.Conv_DoubleToText` _output_get "HalfToEven"))))

(event `self.TimeUp.OnInputTouchBegin`
  (params (FingerIndex :type "ETouchIndex Enum" :default "Touch1") (TouchedComponent :type "PrimitiveComponent Object Reference"))
  ;[1 1 1] 진동 시간 조절
  (set `self.current_Button` TouchedComponent))

(event `self.TimeDown.OnInputTouchEnd`
  (params (FingerIndex :type "ETouchIndex Enum" :default "Touch1") (TouchedComponent :type "PrimitiveComponent Object Reference"))
  ;[1 1 1] 진동 시간 조절
  (if (== TouchedComponent (`self.current_Button`))
    (bind _output_get (set `self.time` (- (`self.time`) 0.1)))
    (`TextRenderComponent.K2_SetText` (`self.Time_Text`) (`KismetTextLibrary.Conv_DoubleToText` _output_get "HalfToEven"))))

(event `self.TimeDown.OnInputTouchBegin`
  (params (FingerIndex :type "ETouchIndex Enum" :default "Touch1") (TouchedComponent :type "PrimitiveComponent Object Reference"))
  ;[1 1 1] 진동 시간 조절
  (set `self.current_Button` TouchedComponent))

(event `self.LeftLarge_Button.OnInputTouchEnd`
  (params (FingerIndex :type "ETouchIndex Enum" :default "Touch1") (TouchedComponent :type "PrimitiveComponent Object Reference"))
  ;[1 1 1] 진동 범위 조절
  (if (== TouchedComponent (`self.current_Button`))
    (if (`self.leftLarge`)
      (set `self.leftLarge` false)
      (`PaperSpriteComponent.SetSpriteColor` (`self.LeftLarge_Button`) (struct :`R` 1.0 :`G` 1.0 :`B` 1.0 :`A` 1.0))
      (else
        (set `self.leftLarge` true)
        (`PaperSpriteComponent.SetSpriteColor` (`self.LeftLarge_Button`) (struct :`R` 1.0 :`A` 1.0))))))

(event `self.LeftLarge_Button.OnInputTouchBegin`
  (params (FingerIndex :type "ETouchIndex Enum" :default "Touch1") (TouchedComponent :type "PrimitiveComponent Object Reference"))
  ;[1 1 1] 진동 범위 조절
  (set `self.current_Button` TouchedComponent))

(event `self.RightLarge_Button.OnInputTouchEnd`
  (params (FingerIndex :type "ETouchIndex Enum" :default "Touch1") (TouchedComponent :type "PrimitiveComponent Object Reference"))
  ;[1 1 1] 진동 범위 조절
  (if (== TouchedComponent (`self.current_Button`))
    (if (`self.rightLarge`)
      (set `self.rightLarge` false)
      (`PaperSpriteComponent.SetSpriteColor` (`self.RightLarge_Button`) (struct :`R` 1.0 :`G` 1.0 :`B` 1.0 :`A` 1.0))
      (else
        (set `self.rightLarge` true)
        (`PaperSpriteComponent.SetSpriteColor` (`self.RightLarge_Button`) (struct :`R` 1.0 :`A` 1.0))))))

(event `self.RightLarge_Button.OnInputTouchBegin`
  (params (FingerIndex :type "ETouchIndex Enum" :default "Touch1") (TouchedComponent :type "PrimitiveComponent Object Reference"))
  ;[1 1 1] 진동 범위 조절
  (set `self.current_Button` TouchedComponent))

(event `self.RightSmall_Button.OnInputTouchEnd`
  (params (FingerIndex :type "ETouchIndex Enum" :default "Touch1") (TouchedComponent :type "PrimitiveComponent Object Reference"))
  ;[1 1 1] 진동 범위 조절
  (if (== TouchedComponent (`self.current_Button`))
    (if (`self.rightSmall`)
      (set `self.rightSmall` false)
      (`PaperSpriteComponent.SetSpriteColor` (`self.RightSmall_Button`) (struct :`R` 1.0 :`G` 1.0 :`B` 1.0 :`A` 1.0))
      (else
        (set `self.rightSmall` true)
        (`PaperSpriteComponent.SetSpriteColor` (`self.RightSmall_Button`) (struct :`R` 1.0 :`A` 1.0))))))

(event `self.RightSmall_Button.OnInputTouchBegin`
  (params (FingerIndex :type "ETouchIndex Enum" :default "Touch1") (TouchedComponent :type "PrimitiveComponent Object Reference"))
  ;[1 1 1] 진동 범위 조절
  (set `self.current_Button` TouchedComponent))

(event `self.LeftSmall_Button.OnInputTouchEnd`
  (params (FingerIndex :type "ETouchIndex Enum" :default "Touch1") (TouchedComponent :type "PrimitiveComponent Object Reference"))
  ;[1 1 1] 진동 범위 조절
  (if (== TouchedComponent (`self.current_Button`))
    (if (`self.leftSmall`)
      (set `self.leftSmall` false)
      (`PaperSpriteComponent.SetSpriteColor` (`self.LeftSmall_Button`) (struct :`R` 1.0 :`G` 1.0 :`B` 1.0 :`A` 1.0))
      (else
        (set `self.leftSmall` true)
        (`PaperSpriteComponent.SetSpriteColor` (`self.LeftSmall_Button`) (struct :`R` 1.0 :`G` 0.005 :`B` 0.005 :`A` 1.0))))))

(event `self.LeftSmall_Button.OnInputTouchBegin`
  (params (FingerIndex :type "ETouchIndex Enum" :default "Touch1") (TouchedComponent :type "PrimitiveComponent Object Reference"))
  ;[1 1 1] 진동 범위 조절
  (set `self.current_Button` TouchedComponent))

(event `self.MainMenu_Button.OnInputTouchEnd`
  (params (FingerIndex :type "ETouchIndex Enum" :default "Touch1") (TouchedComponent :type "PrimitiveComponent Object Reference"))
  ;[1 1 1] 돌아가기
  (if (== TouchedComponent (`self.current_Button`))
    (message `/Game/Blueprints/GameManagerInterface.CallScene_Main` (`self.gameManager`))))

(event `self.MainMenu_Button.OnInputTouchBegin`
  (params (FingerIndex :type "ETouchIndex Enum" :default "Touch1") (TouchedComponent :type "PrimitiveComponent Object Reference"))
  ;[1 1 1] 돌아가기
  (set `self.current_Button` TouchedComponent))

(fn `UserConstructionScript`)