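; A sprite-based progress bar actor that draws its fill from Paper2D components in a configurable gauge color.
; The construction script tints the background and percent bar sprites with their respective colors.
; ProgressBarWorking stores the percent and, when its floored 0–100 value is nonzero, spawns evenly spaced gauge-colored sprites along X under the root.
; Each call adds new sprites without removing earlier ones.
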(event `self.ReceiveBeginPlay`)

(event `self.ReceiveActorBeginOverlap`
  (params (OtherActor :type "Actor Object Reference")))

(event `self.ReceiveTick`
  (params (DeltaSeconds :type "Float (single-precision)")))

(event `ProgressBarWorking`
  (params (percent :type "Float (double-precision)"))
  (bind _returnvalue (`KismetMathLibrary.FFloor` (* 100 (`self.percent`))))
  (set `self.percent` percent)
  (if (`KismetMathLibrary.Conv_IntToBool` _returnvalue)
    (for _index (range (+ _returnvalue 1))
      (bind _returnvalue_2 (`AddComponent|Paper Sprite Component_2` :`bManualAttachment` true))
      (`SceneComponent.K2_AttachTo` _returnvalue_2 (`self.root`) "None" "KeepRelativeOffset" true)
      (`SceneComponent.K2_SetRelativeLocation` _returnvalue_2 (`KismetMathLibrary.MakeVector` (`KismetMathLibrary.Conv_IntToDouble` (- (* _index 32) 1584)) 10.0) false false)
      (`PaperSpriteComponent.SetSpriteColor` _returnvalue_2 (`self.gaugeColor`)))))

(event `Custom Event_0`)

(fn `UserConstructionScript`
  (`PaperSpriteComponent.SetSpriteColor` (`self.BGBar`) (`self.BGColor`))
  (`PaperSpriteComponent.SetSpriteColor` (`self.PercentBar`) (`self.gaugeColor`)))