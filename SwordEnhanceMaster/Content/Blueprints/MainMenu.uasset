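; Main menu actor with touch buttons for game start, new game and continue, each firing only when touch begins and ends on the same component.
; Start slides the interface background sideways via a timeline with collision disabled.
; New game asks for confirmation through CheckWindowActor if a save exists; a yes answer resets GameManager data from a fresh GameSaveData.
; Continue loads the save slot into GameManager, which handles the home scene transition.
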(event `self.GameStart_Button.OnInputTouchEnd`
  (params (FingerIndex :type "ETouchIndex Enum" :default "Touch1") (TouchedComponent :type "PrimitiveComponent Object Reference"))
  ;[1 1 1] 게임시작버튼
  (if (== TouchedComponent (`self.enableButton`))
    (`self.SetActorEnableCollision` false)
    (set `self.originalLocation` (`SceneComponent.K2_GetComponentLocation` (`self.InterfaceBG_Sprite`)))
    (bind (_direction `_인터페이스_이동`) (`Timeline|인터페이스 이동` :!via `PlayFromStart`)
      (:`Update`
        (`SceneComponent.K2_SetWorldLocation` (`self.InterfaceBG_Sprite`) (+ (`KismetMathLibrary.MakeVector` (* `_인터페이스_이동` -900.0)) (`self.originalLocation`)) false false))
      (:`Finished`
        (`self.SetActorEnableCollision` true)))))

(event `self.GameStart_Button.OnInputTouchBegin`
  (params (FingerIndex :type "ETouchIndex Enum" :default "Touch1") (TouchedComponent :type "PrimitiveComponent Object Reference"))
  ;[1 1 1] 게임시작버튼
  (set `self.enableButton` TouchedComponent))

(event `self.NewStart_Button.OnInputTouchEnd`
  (params (FingerIndex :type "ETouchIndex Enum" :default "Touch1") (TouchedComponent :type "PrimitiveComponent Object Reference"))
  ;[1 1 1] 새로하기버튼
  (if (== TouchedComponent (`self.enableButton`))
    (bind _returnvalue (`GameplayStatics.DoesSaveGameExist` "GameSaveSlot1"))
    (if _returnvalue
      (set `self.currentAction` "NewEnumerator0")
      (message `/Game/Blueprints/WindowManager.CallWindow` (`self.checkWindow_Actor`) "데이터가 이미 존재하고 있습니다.<br>정말 새로 하시겠습니까" self)
      (else
        (message `/Game/Blueprints/GameManagerInterface.CreateSaveFile` (`self.gameManager`))
        (message `/Game/Blueprints/GameManagerInterface.CallScene_Home` (`self.gameManager`))))))

(event `self.NewStart_Button.OnInputTouchBegin`
  (params (FingerIndex :type "ETouchIndex Enum" :default "Touch1") (TouchedComponent :type "PrimitiveComponent Object Reference"))
  ;[1 1 1] 새로하기버튼
  (set `self.enableButton` TouchedComponent))

(event `self.Continue_Button.OnInputTouchEnd`
  (params (FingerIndex :type "ETouchIndex Enum" :default "Touch1") (TouchedComponent :type "PrimitiveComponent Object Reference"))
  ;[1 1 1] 이어하기버튼
  (if (== TouchedComponent (`self.enableButton`))
    (bind _returnvalue (`GameplayStatics.DoesSaveGameExist` "GameSaveSlot1"))
    (if _returnvalue
      (bind _returnvalue_2 (`GameplayStatics.LoadGameFromSlot` "GameSaveSlot1"))
      (bind _asgame_save_data (cast `/Game/Blueprints/GameSetting/GameSaveData` _returnvalue_2))
      (set `/Game/Blueprints/GameManager.gameSaveDataObject` _asgame_save_data (`self.gameManager`))
      (message `/Game/Blueprints/GameManagerInterface.CallScene_Home` (`self.gameManager`))
      (else
        (`KismetSystemLibrary.PrintString` "No Data")))))

(event `self.Continue_Button.OnInputTouchBegin`
  (params (FingerIndex :type "ETouchIndex Enum" :default "Touch1") (TouchedComponent :type "PrimitiveComponent Object Reference"))
  ;[1 1 1] 이어하기버튼
  (set `self.enableButton` TouchedComponent))

(event `/Game/Blueprints/WindowManager.SendButtonEvent`
  (params (Answer :type Boolean))
  ;[0.965 1 0.9887] 새로하기 버튼 이벤트 (이전 게임 데이터 존재)
  (switch `/Game/Blueprints/ActionList` (`self.currentAction`)
    (:`NewEnumerator0`
      (if Answer
        ;;[0.3796 0.6515 0.8] Yes버튼 이벤트 - 게임 데이터 초기화
        (bind _returnvalue (`GameplayStatics.CreateSaveGameObject` "/Game/Blueprints/GameSetting/GameSaveData.GameSaveData_C"))
        (bind _asgame_save_data (cast `/Game/Blueprints/GameSetting/GameSaveData` _returnvalue))
        (bind _output_get (set `/Game/Blueprints/GameManager.gameSaveDataObject` _asgame_save_data (`self.gameManager`)))
        (for (_array_element _array_index) (`/Game/Blueprints/GameSetting/GameSaveData.swordInfo` (`/Game/Blueprints/GameManager.gameSaveDataObject` (`self.gameManager`)))
          (`KismetArrayLibrary.Array_Set` (`/Game/Blueprints/GameManager.swordInfo` (`self.gameManager`)) _array_index _array_element true))
        (for (_array_element_2 _array_index_2) (`/Game/Blueprints/GameSetting/GameSaveData.ingredientInfo` (`/Game/Blueprints/GameManager.gameSaveDataObject` (`self.gameManager`)))
          (`KismetArrayLibrary.Array_Set` (`/Game/Blueprints/GameManager.ingredientInfo` (`self.gameManager`)) _array_index_2 _array_element_2 true)
          (set `/Game/Blueprints/GameManager.labLevel` (`/Game/Blueprints/GameSetting/GameSaveData.labLevel` (`/Game/Blueprints/GameManager.gameSaveDataObject` (`self.gameManager`))) (`self.gameManager`))
          (`GameplayStatics.SaveGameToSlot` _output_get "GameSaveSlot1")
          (message `/Game/Blueprints/GameManagerInterface.CallScene_Home` (`self.gameManager`)))
        (else
          ;;[0.3796 0.6515 0.8] No버튼 이벤트 - 메인메뉴로 돌아감
          (`self.SetActorEnableCollision` true))))))

(fn `UserConstructionScript`)