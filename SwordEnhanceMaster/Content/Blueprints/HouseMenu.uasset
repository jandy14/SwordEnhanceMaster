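; House menu actor with touch buttons that slide the interface between enhancement and laboratory screens and open weapon and ingredient inventories.
; Button presses count only when release matches the touched component; timelines move the background sideways with collision disabled during the slide.
; SelectItem receives a weapon index, hides the inventory, then fills the sprite, stats from the SwordList data table, and enhancement levels and name from the game manager.
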(event `self.GoInhance_Button.OnInputTouchEnd`
  (params (FingerIndex :type "ETouchIndex Enum" :default "Touch1") (TouchedComponent :type "PrimitiveComponent Object Reference"))
  ;[1 1 1] 강화 메뉴 버튼
  (if (== TouchedComponent (`self.enableButton`))
    (`self.SetActorEnableCollision` false)
    (set `self.originalLocation` (`SceneComponent.K2_GetComponentLocation` (`self.HouseInterfaceBG`)))
    (bind (_direction `_인터페이스_이동`) (`Timeline|강화메뉴로` :!via `PlayFromStart`)
      (:`Update`
        (`SceneComponent.K2_SetWorldLocation` (`self.HouseInterfaceBG`) (+ (`KismetMathLibrary.MakeVector` (* `_인터페이스_이동` -900.0)) (`self.originalLocation`)) false false))
      (:`Finished`
        (`self.SetActorEnableCollision` true)))))

(event `self.GoInhance_Button.OnInputTouchBegin`
  (params (FingerIndex :type "ETouchIndex Enum" :default "Touch1") (TouchedComponent :type "PrimitiveComponent Object Reference"))
  ;[1 1 1] 강화 메뉴 버튼
  (set `self.enableButton` TouchedComponent))

(event `self.GoLaboratory_Button.OnInputTouchEnd`
  (params (FingerIndex :type "ETouchIndex Enum" :default "Touch1") (TouchedComponent :type "PrimitiveComponent Object Reference"))
  ;[1 1 1] 연구 메뉴 버튼
  (if (== TouchedComponent (`self.enableButton`))
    (`self.SetActorEnableCollision` false)
    (set `self.originalLocation` (`SceneComponent.K2_GetComponentLocation` (`self.HouseInterfaceBG`)))
    (bind (_direction `_인터페이스_이동`) (`Timeline|연구메뉴로` :!via `PlayFromStart`)
      (:`Update`
        (`SceneComponent.K2_SetWorldLocation` (`self.HouseInterfaceBG`) (+ (`KismetMathLibrary.MakeVector` (* `_인터페이스_이동` 900.0)) (`self.originalLocation`)) false false))
      (:`Finished`
        (`self.SetActorEnableCollision` true)))))

(event `self.GoLaboratory_Button.OnInputTouchBegin`
  (params (FingerIndex :type "ETouchIndex Enum" :default "Touch1") (TouchedComponent :type "PrimitiveComponent Object Reference"))
  ;[1 1 1] 연구 메뉴 버튼
  (set `self.enableButton` TouchedComponent))

(event `self.WeaponCollision.OnInputTouchEnd`
  (params (FingerIndex :type "ETouchIndex Enum" :default "Touch1") (TouchedComponent :type "PrimitiveComponent Object Reference"))
  ;[1 1 1] 무기창 호출
  (if (== TouchedComponent (`self.enableButton`))
    (message `/Game/Blueprints/InventoryManager.ShowInventory` (`self.weaponInventory_Actor`) self)))

(event `/Game/Blueprints/InventoryManager.SelectItem`
  (params (Index :type Integer))
  (bind (_item_swordname _item_swordnumber `_item_소재강화` `_item_예리함강화` `_item_무게감강화` `_item_속성강화`) (break `/Game/Blueprints/SwordInfo` (`KismetArrayLibrary.Array_Get` (`/Game/Blueprints/GameManager.swordInfo` (`self.actor_GameManager`)) Index)))
  ;[1 1 1] 강화할 무기 선택 이벤트
  (`SceneComponent.SetHiddenInGame` (`self.Text_Sharpness`) false false)
  (`SceneComponent.SetHiddenInGame` (`self.Text_Mass`) false false)
  (`SceneComponent.SetHiddenInGame` (`self.Text_Material`) false false)
  (`SceneComponent.SetHiddenInGame` (`self.Text_Name`) false false)
  (`SceneComponent.SetHiddenInGame` (`self.Text_Attack`) false false)
  (`SceneComponent.SetHiddenInGame` (`self.Text_Speed`) false false)
  (`SceneComponent.SetHiddenInGame` (`self.Text_Critical`) false false)
  (`SceneComponent.SetHiddenInGame` (`self.Text_CriticalPercent`) false false)
  (`SceneComponent.SetHiddenInGame` (`self.Text_Defense`) false false)
  (`|ExecutionSequence`
    (:`then_0`
      (`PaperSpriteComponent.SetSprite` (`self.WeaponImage`) (`KismetArrayLibrary.Array_Get` (`/Game/Blueprints/GameManager.swordSprite_Array` (`self.actor_GameManager`)) (`KismetStringLibrary.Conv_StringToInt` (`KismetStringLibrary.Conv_NameToString` _item_swordnumber))))
      (`SceneComponent.SetWorldScale3D` (`self.WeaponImage`) (0.4 0.4 0.4))
      (`self.SetActorHiddenInGame` (`self.weaponInventory_Actor`) true)
      (`self.SetActorEnableCollision` (`self.weaponInventory_Actor`) false)
      (`self.SetActorEnableCollision` true)
      (bind _returnvalue (`|GetDataTableRow` "/Game/Blueprints/SwordList.SwordList" _item_swordnumber)
        (:`then`
          (`|ExecutionSequence`
            (:`then_0`
              (bind (_swordname _swordpower _swordspeed _criticalrate _criticaldamege _defenserate) (break `/Game/Blueprints/SwordStruct` _returnvalue))
              (`TextRenderComponent.K2_SetText` (`self.Text_Attack`) (`KismetTextLibrary.Conv_StringToText` (`KismetStringLibrary.Concat_StrStr` "공격력 : " (`KismetStringLibrary.Conv_IntToString` _swordpower)))))
            (:`then_1`
              (`TextRenderComponent.K2_SetText` (`self.Text_Speed`) (`KismetTextLibrary.Conv_StringToText` (`KismetStringLibrary.Concat_StrStr` "공격 속도 : " (`KismetStringLibrary.Conv_DoubleToString` _swordspeed)))))
            (:`then_2`
              (`TextRenderComponent.K2_SetText` (`self.Text_Critical`) (`KismetTextLibrary.Conv_StringToText` (`KismetStringLibrary.Concat_StrStr` "크리티컬 데미지 : " (`KismetStringLibrary.Conv_DoubleToString` _criticaldamege)))))
            (:`then_3`
              (`TextRenderComponent.K2_SetText` (`self.Text_CriticalPercent`) (`KismetTextLibrary.Conv_StringToText` (`KismetStringLibrary.Concat_StrStr` "크리티컬 확률 : " (`KismetStringLibrary.Conv_DoubleToString` _criticalrate)))))
            (:`then_4`
              (`TextRenderComponent.K2_SetText` (`self.Text_Defense`) (`KismetTextLibrary.Conv_StringToText` (`KismetStringLibrary.Concat_StrStr` "방어 확률 : " (`KismetStringLibrary.Conv_DoubleToString` _defenserate)))))))))
    (:`then_1`
      (`TextRenderComponent.K2_SetText` (`self.Text_Sharpness`) (`KismetTextLibrary.Conv_StringToText` (`KismetStringLibrary.Concat_StrStr` "예+" (`KismetStringLibrary.Conv_IntToString` `_item_예리함강화`))))
      (`TextRenderComponent.K2_SetText` (`self.Text_Mass`) (`KismetTextLibrary.Conv_StringToText` (`KismetStringLibrary.Concat_StrStr` "무+" (`KismetStringLibrary.Conv_IntToString` `_item_무게감강화`))))
      (`TextRenderComponent.K2_SetText` (`self.Text_Material`) (`KismetTextLibrary.Conv_StringToText` (`KismetStringLibrary.Concat_StrStr` "소+" (`KismetStringLibrary.Conv_IntToString` `_item_소재강화`))))
      (if (`KismetTextLibrary.EqualEqual_TextText` `_item_속성강화` "null")
        (`TextRenderComponent.K2_SetText` (`self.Text_Name`) _item_swordname)
        (else
          (`TextRenderComponent.K2_SetText` (`self.Text_Name`) (`KismetTextLibrary.Conv_StringToText` (`KismetStringLibrary.Concat_StrStr` (`KismetTextLibrary.Conv_TextToString` `_item_속성강화`) " " (`KismetTextLibrary.Conv_TextToString` _item_swordname)))))))))

(event `self.WeaponCollision.OnInputTouchBegin`
  (params (FingerIndex :type "ETouchIndex Enum" :default "Touch1") (TouchedComponent :type "PrimitiveComponent Object Reference"))
  ;[1 1 1] 무기창 호출
  (set `self.enableButton` TouchedComponent))

(event `self.IngredientCollision.OnInputTouchEnd`
  (params (FingerIndex :type "ETouchIndex Enum" :default "Touch1") (TouchedComponent :type "PrimitiveComponent Object Reference"))
  ;[1 1 1] 재료창 호출
  (if (== TouchedComponent (`self.enableButton`))
    (message `/Game/Blueprints/InventoryManager.ShowIngredientInventory` (`self.ingredientInventory_Actor`) self)))

(event `self.IngredientCollision.OnInputTouchBegin`
  (params (FingerIndex :type "ETouchIndex Enum" :default "Touch1") (TouchedComponent :type "PrimitiveComponent Object Reference"))
  ;[1 1 1] 재료창 호출
  (set `self.enableButton` TouchedComponent))

(fn `UserConstructionScript`)