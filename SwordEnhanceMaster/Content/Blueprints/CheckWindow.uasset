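; CheckWindow is a touch-driven Yes/No confirmation popup actor.
; CallWindow stores the calling scene, sets the prompt text, shows the window and disables the scene's collision while it is open.
; A button only fires when touch end lands on the component recorded at touch begin.
; Either answer hides the window, re-enables the scene's collision and sends the boolean result back through SendButtonEventMessage.
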(event `self.Yes_Button.OnInputTouchEnd`
  (params (FingerIndex :type "ETouchIndex Enum" :default "Touch1") (TouchedComponent :type "PrimitiveComponent Object Reference"))
  ;[1 1 1] Yes버튼 이벤트
  (if (== TouchedComponent (`self.currentButton`))
    (set `self.checkWindow` true)
    (`self.SetActorHiddenInGame` true)
    (`self.SetActorEnableCollision` false)
    (`self.SetActorEnableCollision` (`self.attachToScene`) true)
    (message `/Game/Blueprints/WindowManager.SendButtonEvent` (`self.attachToScene`) (`self.checkWindow`))))

(event `self.Yes_Button.OnInputTouchBegin`
  (params (FingerIndex :type "ETouchIndex Enum" :default "Touch1") (TouchedComponent :type "PrimitiveComponent Object Reference"))
  ;[1 1 1] Yes버튼 이벤트
  (set `self.currentButton` TouchedComponent))

(event `self.No_Button.OnInputTouchEnd`
  (params (FingerIndex :type "ETouchIndex Enum" :default "Touch1") (TouchedComponent :type "PrimitiveComponent Object Reference"))
  ;[1 1 1] No버튼 이벤트
  (if (== TouchedComponent (`self.currentButton`))
    (set `self.checkWindow` false)
    (`self.SetActorHiddenInGame` true)
    (`self.SetActorEnableCollision` false)
    (`self.SetActorEnableCollision` (`self.attachToScene`) true)
    (message `/Game/Blueprints/WindowManager.SendButtonEvent` (`self.attachToScene`) (`self.checkWindow`))))

(event `self.No_Button.OnInputTouchBegin`
  (params (FingerIndex :type "ETouchIndex Enum" :default "Touch1") (TouchedComponent :type "PrimitiveComponent Object Reference"))
  ;[1 1 1] No버튼 이벤트
  (set `self.currentButton` TouchedComponent))

(event `/Game/Blueprints/WindowManager.CallWindow`
  (params (Text :type String) (Scene :type "Actor Object Reference"))
  ;[1 1 1] Check Window 호출
  (set `self.attachToScene` Scene)
  (`TextRenderComponent.K2_SetText` (`self.MainText`) (`KismetTextLibrary.Conv_StringToText` Text))
  (`self.SetActorEnableCollision` true)
  (`self.SetActorHiddenInGame` false)
  (`self.SetActorEnableCollision` (`self.attachToScene`) false))

(fn `UserConstructionScript`)