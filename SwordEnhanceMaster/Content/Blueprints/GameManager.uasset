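; GameManager is the actor that sets up the game at start and handles the switch to the home scene.
; BeginPlay makes itself the view target, copies sword, ingredient and lab-level data from the save slot if present, then hides inventories, check window and house menu.
; CallSceneHome swaps scenes by toggling visibility and collision on placed actors rather than loading levels.
; CreateSaveFile writes a fresh GameSaveData to the slot without copying current values.
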(event `self.ReceiveBeginPlay`
  (bind (_returnvalue_x _returnvalue_y) (`KismetMathLibrary.BreakVector2D` (`WidgetLayoutLibrary.GetViewportSize`)))
  ;[1 1 1] 카메라 세팅
  (`PlayerController.SetViewTargetWithBlend` (`GameplayStatics.GetPlayerController` 0) self 0.0 "VTBlend_Linear" 0.0 false)
  (`KismetSystemLibrary.PrintString` (`KismetStringLibrary.Conv_DoubleToString` _returnvalue_x))
  (`KismetSystemLibrary.PrintString` (`KismetStringLibrary.Conv_DoubleToString` _returnvalue_y))
  ;[1 1 1] 세이브 데이터 로드
  (bind _returnvalue (`GameplayStatics.DoesSaveGameExist` "GameSaveSlot1"))
  (if _returnvalue
    (bind _returnvalue_2 (`GameplayStatics.LoadGameFromSlot` "GameSaveSlot1"))
    (bind _asgame_save_data (cast `/Game/Blueprints/GameSetting/GameSaveData` _returnvalue_2))
    (bind _output_get (set `self.gameSaveDataObject` _asgame_save_data))
    (for (_array_element _array_index) (`/Game/Blueprints/GameSetting/GameSaveData.swordInfo` _output_get)
      (`KismetArrayLibrary.Array_Set` (`self.swordInfo`) _array_index _array_element true))
    (for (_array_element_2 _array_index_2) (`/Game/Blueprints/GameSetting/GameSaveData.ingredientInfo` (`self.gameSaveDataObject`))
      (`KismetArrayLibrary.Array_Set` (`self.ingredientInfo`) _array_index_2 _array_element_2 true))
    (set `self.labLevel` (`/Game/Blueprints/GameSetting/GameSaveData.labLevel` (`self.gameSaveDataObject`))))
  ;[1 1 1] 인벤토리 비활성화
  (`self.SetActorHiddenInGame` (`self.actor_Inventory`) true)
  (`self.SetActorEnableCollision` (`self.actor_Inventory`) false)
  (`self.SetActorHiddenInGame` (`self.ingredientInventory_Actor`) true)
  (`self.SetActorEnableCollision` (`self.ingredientInventory_Actor`) false)
  ;[1 1 1] CheckWindow 비활성화
  (`self.SetActorHiddenInGame` (`self.actor_CheckWindow`) true)
  (`self.SetActorEnableCollision` (`self.actor_CheckWindow`) false)
  ;[1 1 1] Text 비활성화
  (`SceneComponent.SetHiddenInGame` (`/Game/Blueprints/HouseMenu.Text_Sharpness` (`self.houseMenu`)) true false)
  (`SceneComponent.SetHiddenInGame` (`/Game/Blueprints/HouseMenu.Text_Mass` (`self.houseMenu`)) true false)
  (`SceneComponent.SetHiddenInGame` (`/Game/Blueprints/HouseMenu.Text_Material` (`self.houseMenu`)) true false)
  (`SceneComponent.SetHiddenInGame` (`/Game/Blueprints/HouseMenu.Text_Name` (`self.houseMenu`)) true false)
  (`SceneComponent.SetHiddenInGame` (`/Game/Blueprints/HouseMenu.Text_Attack` (`self.houseMenu`)) true false)
  (`SceneComponent.SetHiddenInGame` (`/Game/Blueprints/HouseMenu.Text_Speed` (`self.houseMenu`)) true false)
  (`SceneComponent.SetHiddenInGame` (`/Game/Blueprints/HouseMenu.Text_Critical` (`self.houseMenu`)) true false)
  (`SceneComponent.SetHiddenInGame` (`/Game/Blueprints/HouseMenu.Text_CriticalPercent` (`self.houseMenu`)) true false)
  (`SceneComponent.SetHiddenInGame` (`/Game/Blueprints/HouseMenu.Text_Defense` (`self.houseMenu`)) true false)
  ;[1 1 1] Scene 비활성화
  (`self.SetActorEnableCollision` (`self.houseMenu`) false)
  (`self.SetActorHiddenInGame` (`self.houseMenu`) true))

(event `/Game/Blueprints/GameManagerInterface.CallScene_Home`
  ;[1 1 1] HouseMenu Scene 호출
  (`self.SetActorHiddenInGame` (`self.currentScene`) true)
  (`self.SetActorEnableCollision` (`self.currentScene`) false)
  (`self.SetActorHiddenInGame` (`self.houseMenu`) false)
  (`self.SetActorEnableCollision` (`self.houseMenu`) true)
  (set `self.currentScene` (`self.houseMenu`)))

(event `/Game/Blueprints/GameManagerInterface.CreateSaveFile`
  ;[1 1 1] 세이브 파일 생성
  (bind _returnvalue (`GameplayStatics.CreateSaveGameObject` "/Game/Blueprints/GameSetting/GameSaveData.GameSaveData_C"))
  (bind _asgame_save_data (cast `/Game/Blueprints/GameSetting/GameSaveData` _returnvalue))
  (bind _output_get (set `self.GameSaveDataObject` _asgame_save_data))
  (`GameplayStatics.SaveGameToSlot` _output_get "GameSaveSlot1"))

(fn `UserConstructionScript`)