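; Touch-driven weapon inventory actor that shows the player's saved swords four per page for selection.
; ShowInventory blocks collision on the calling scene actor, computes the page count from the save data's SwordInfo and refreshes slot sprites, hiding empty slots.
; Tapping a slot sends its absolute index to that scene via SelectItemMessage, then closes and restores its collision.
; Buttons fire only when touch begins and ends on the same component.
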(event `self.CloseButton_Sprite.OnInputTouchEnd`
  (params (FingerIndex :type "ETouchIndex Enum" :default "Touch1") (TouchedComponent :type "PrimitiveComponent Object Reference"))
  ;[1 1 1] 닫기 버튼 이벤트
  (if (== TouchedComponent (`self.enableButton`))
    (`self.CloseInventory`)))

(event `self.CloseButton_Sprite.OnInputTouchBegin`
  (params (FingerIndex :type "ETouchIndex Enum" :default "Touch1") (TouchedComponent :type "PrimitiveComponent Object Reference"))
  ;[1 1 1] 닫기 버튼 이벤트
  (set `self.enableButton` TouchedComponent))

(event `/Game/Blueprints/InventoryManager.SetItemSlot`
  (bind _infoslot1 (`self.InfoSlot1`))
  (bind _infoslot1_2 (`self.InfoSlot1`))
  (bind _inventoryslot2 (`self.InventorySlot2`))
  (bind _inventoryslot3 (`self.InventorySlot3`))
  (bind _swordimage1 (`self.SwordImage1`))
  (bind _inventoryslot2_2 (`self.InventorySlot2`))
  (bind _inventoryslot3_2 (`self.InventorySlot3`))
  (bind _inventoryslot4 (`self.InventorySlot4`))
  ;[1 1 1] 아이템 슬롯 세팅
  (for _index (range (- (* (`self.nowPage`) 4) 4) (* (`self.nowPage`) 4))
    (if (> (`KismetArrayLibrary.Array_Length` (`/Game/Blueprints/GameSetting/GameSaveData.swordInfo` (`/Game/Blueprints/GameManager.gameSaveDataObject` (`self.gameManager`)))) _index)
      (bind _returnvalue (mod _index 4))
      ;;[1 1 1] 아이템 Sprite 적용
      (switch `int` _returnvalue
        (:`0`
          (bind _item (`KismetArrayLibrary.Array_Get` (`/Game/Blueprints/GameManager.swordSprite_Array` (`self.gameManager`)) (`KismetStringLibrary.Conv_StringToInt` (`KismetStringLibrary.Conv_NameToString` (`.swordNumber_40_1B7337BC4CA4F1335FCEDA976FA4A7CA` (break `/Game/Blueprints/SwordInfo` (`KismetArrayLibrary.Array_Get` (`/Game/Blueprints/GameSetting/GameSaveData.swordInfo` (`/Game/Blueprints/GameManager.gameSaveDataObject` (`self.gameManager`))) _index)))))))
          (`PaperSpriteComponent.SetSprite` _swordimage1 _item)
          (`SceneComponent.SetVisibility` _infoslot1 true false)
          (`SceneComponent.SetVisibility` (`self.InventorySlot1`) true false)
          (`SceneComponent.SetVisibility` (`self.SwordImage1`) true false)
          (`SceneComponent.SetVisibility` (`self.SlotCollision1`) true false)
          (`PrimitiveComponent.SetCollisionEnabled` _infoslot1 "QueryAndPhysics")
          (`PrimitiveComponent.SetCollisionEnabled` (`self.InventorySlot1`) "QueryAndPhysics")
          (`PrimitiveComponent.SetCollisionEnabled` (`self.SwordImage1`) "QueryAndPhysics")
          (`PrimitiveComponent.SetCollisionEnabled` (`self.SlotCollision1`) "QueryAndPhysics"))
        (:`1`
          (`PaperSpriteComponent.SetSprite` (`self.SwordImage2`) _item)
          (`SceneComponent.SetVisibility` _inventoryslot2_2 true false)
          (`SceneComponent.SetVisibility` (`self.InfoSlot2`) true false)
          (`SceneComponent.SetVisibility` (`self.SwordImage2`) true false)
          (`SceneComponent.SetVisibility` (`self.SlotCollision2`) true false)
          (`PrimitiveComponent.SetCollisionEnabled` _inventoryslot2_2 "QueryAndPhysics")
          (`PrimitiveComponent.SetCollisionEnabled` (`self.InfoSlot2`) "QueryAndPhysics")
          (`PrimitiveComponent.SetCollisionEnabled` (`self.SwordImage2`) "QueryAndPhysics")
          (`PrimitiveComponent.SetCollisionEnabled` (`self.SlotCollision2`) "QueryAndPhysics"))
        (:`2`
          (`PaperSpriteComponent.SetSprite` (`self.SwordImage3`) _item)
          (`SceneComponent.SetVisibility` _inventoryslot3_2 true false)
          (`SceneComponent.SetVisibility` (`self.InfoSlot3`) true false)
          (`SceneComponent.SetVisibility` (`self.SwordImage3`) true false)
          (`SceneComponent.SetVisibility` (`self.SlotCollision3`) true false)
          (`PrimitiveComponent.SetCollisionEnabled` _inventoryslot3_2 "QueryAndPhysics")
          (`PrimitiveComponent.SetCollisionEnabled` (`self.InfoSlot3`) "QueryAndPhysics")
          (`PrimitiveComponent.SetCollisionEnabled` (`self.SwordImage3`) "QueryAndPhysics")
          (`PrimitiveComponent.SetCollisionEnabled` (`self.SlotCollision3`) "QueryAndPhysics"))
        (:`3`
          (`PaperSpriteComponent.SetSprite` (`self.SwordImage4`) _item)
          (`SceneComponent.SetVisibility` _inventoryslot4 true false)
          (`SceneComponent.SetVisibility` (`self.InfoSlot4`) true false)
          (`SceneComponent.SetVisibility` (`self.SwordImage4`) true false)
          (`SceneComponent.SetVisibility` (`self.SlotCollision4`) true false)
          (`PrimitiveComponent.SetCollisionEnabled` _inventoryslot4 "QueryAndPhysics")
          (`PrimitiveComponent.SetCollisionEnabled` (`self.InfoSlot4`) "QueryAndPhysics")
          (`PrimitiveComponent.SetCollisionEnabled` (`self.SwordImage4`) "QueryAndPhysics")
          (`PrimitiveComponent.SetCollisionEnabled` (`self.SlotCollision4`) "QueryAndPhysics")))
      (`SceneComponent.SetWorldScale3D` _swordimage1 (0.4 0.4 0.4))
      (`SceneComponent.SetWorldScale3D` (`self.SwordImage2`) (0.4 0.4 0.4))
      (`SceneComponent.SetWorldScale3D` (`self.SwordImage3`) (0.4 0.4 0.4))
      (`SceneComponent.SetWorldScale3D` (`self.SwordImage4`) (0.4 0.4 0.4))
      (else
        ;;[1 1 1] 비어있는 슬롯 비활성화
        (switch `int` _returnvalue
          (:`0`
            (`SceneComponent.SetVisibility` _infoslot1_2 false false)
            (`SceneComponent.SetVisibility` (`self.InventorySlot1`) false false)
            (`SceneComponent.SetVisibility` (`self.SwordImage1`) false false)
            (`SceneComponent.SetVisibility` (`self.SlotCollision1`) false false)
            (`PrimitiveComponent.SetCollisionEnabled` _infoslot1_2 "NoCollision")
            (`PrimitiveComponent.SetCollisionEnabled` (`self.InventorySlot1`) "NoCollision")
            (`PrimitiveComponent.SetCollisionEnabled` (`self.SwordImage1`) "NoCollision")
            (`PrimitiveComponent.SetCollisionEnabled` (`self.SlotCollision1`) "NoCollision"))
          (:`1`
            (`SceneComponent.SetVisibility` _inventoryslot2 false false)
            (`SceneComponent.SetVisibility` (`self.InfoSlot2`) false false)
            (`SceneComponent.SetVisibility` (`self.SwordImage2`) false false)
            (`SceneComponent.SetVisibility` (`self.SlotCollision2`) false false)
            (`PrimitiveComponent.SetCollisionEnabled` _inventoryslot2 "NoCollision")
            (`PrimitiveComponent.SetCollisionEnabled` (`self.InfoSlot2`) "NoCollision")
            (`PrimitiveComponent.SetCollisionEnabled` (`self.SwordImage2`) "NoCollision")
            (`PrimitiveComponent.SetCollisionEnabled` (`self.SlotCollision2`) "NoCollision"))
          (:`2`
            (`SceneComponent.SetVisibility` _inventoryslot3 false false)
            (`SceneComponent.SetVisibility` (`self.InfoSlot3`) false false)
            (`SceneComponent.SetVisibility` (`self.SwordImage3`) false false)
            (`SceneComponent.SetVisibility` (`self.SlotCollision3`) false false)
            (`PrimitiveComponent.SetCollisionEnabled` _inventoryslot3 "NoCollision")
            (`PrimitiveComponent.SetCollisionEnabled` (`self.InfoSlot3`) "NoCollision")
            (`PrimitiveComponent.SetCollisionEnabled` (`self.SwordImage3`) "NoCollision")
            (`PrimitiveComponent.SetCollisionEnabled` (`self.SlotCollision3`) "NoCollision"))
          (:`3`
            (`SceneComponent.SetVisibility` (`self.InventorySlot4`) false false)
            (`SceneComponent.SetVisibility` (`self.InfoSlot4`) false false)
            (`SceneComponent.SetVisibility` (`self.SwordImage4`) false false)
            (`SceneComponent.SetVisibility` (`self.SlotCollision4`) false false)
            (`PrimitiveComponent.SetCollisionEnabled` (`self.InfoSlot4`) "NoCollision")
            (`PrimitiveComponent.SetCollisionEnabled` (`self.InventorySlot4`) "NoCollision")
            (`PrimitiveComponent.SetCollisionEnabled` (`self.SwordImage4`) "NoCollision")
            (`PrimitiveComponent.SetCollisionEnabled` (`self.SlotCollision4`) "NoCollision"))))))
  (`TextRenderComponent.K2_SetText` (`self.TextRender`) (`KismetTextLibrary.Conv_StringToText` (`KismetStringLibrary.Concat_StrStr` (`KismetStringLibrary.Conv_IntToString` (`self.nowPage`)) " of " (`KismetStringLibrary.Conv_IntToString` (`self.maxPage`))))))

(event `self.SlotCollision1.OnInputTouchEnd`
  (params (FingerIndex :type "ETouchIndex Enum" :default "Touch1") (TouchedComponent :type "PrimitiveComponent Object Reference"))
  ;[1 1 1] 아이템 슬롯1 클릭 이벤트
  (if (== TouchedComponent (`self.enableButton`))
    (message `/Game/Blueprints/InventoryManager.SelectItem` (`self.attachToScene`) (+ (* (- (`self.nowPage`) 1) 4) 0))
    (`self.CloseInventory`)))

(event `self.SlotCollision1.OnInputTouchBegin`
  (params (FingerIndex :type "ETouchIndex Enum" :default "Touch1") (TouchedComponent :type "PrimitiveComponent Object Reference"))
  ;[1 1 1] 아이템 슬롯1 클릭 이벤트
  (set `self.enableButton` TouchedComponent))

(event `self.SlotCollision2.OnInputTouchEnd`
  (params (FingerIndex :type "ETouchIndex Enum" :default "Touch1") (TouchedComponent :type "PrimitiveComponent Object Reference"))
  ;[1 1 1] 아이템 슬롯2 클릭 이벤트
  (if (== TouchedComponent (`self.enableButton`))
    (message `/Game/Blueprints/InventoryManager.SelectItem` (`self.attachToScene`) (+ (* (- (`self.nowPage`) 1) 4) 1))
    (`self.CloseInventory`)))

(event `self.SlotCollision2.OnInputTouchBegin`
  (params (FingerIndex :type "ETouchIndex Enum" :default "Touch1") (TouchedComponent :type "PrimitiveComponent Object Reference"))
  ;[1 1 1] 아이템 슬롯2 클릭 이벤트
  (set `self.enableButton` TouchedComponent))

(event `self.SlotCollision3.OnInputTouchEnd`
  (params (FingerIndex :type "ETouchIndex Enum" :default "Touch1") (TouchedComponent :type "PrimitiveComponent Object Reference"))
  ;[1 1 1] 아이템 슬롯3 클릭 이벤트
  (if (== TouchedComponent (`self.enableButton`))
    (message `/Game/Blueprints/InventoryManager.SelectItem` (`self.attachToScene`) (+ (* (- (`self.nowPage`) 1) 4) 2))
    (`self.CloseInventory`)))

(event `self.SlotCollision3.OnInputTouchBegin`
  (params (FingerIndex :type "ETouchIndex Enum" :default "Touch1") (TouchedComponent :type "PrimitiveComponent Object Reference"))
  ;[1 1 1] 아이템 슬롯3 클릭 이벤트
  (set `self.enableButton` TouchedComponent))

(event `/Game/Blueprints/InventoryManager.ShowInventory`
  (params (SceneFrom :type "Actor Object Reference"))
  (bind _returnvalue (`KismetArrayLibrary.Array_Length` (`/Game/Blueprints/GameSetting/GameSaveData.swordInfo` (`/Game/Blueprints/GameManager.gameSaveDataObject` (`self.gameManager`)))))
  (bind _returnvalue_2 (/ _returnvalue 4))
  ;[1 1 1] 무기 인벤토리 활성화
  (bind _output_get (set `self.attachToScene` SceneFrom))
  (`self.SetActorEnableCollision` _output_get false)
  (`self.SetActorHiddenInGame` false)
  (`self.SetActorEnableCollision` true)
  (if (== (mod _returnvalue 4) 0)
    (if (== _returnvalue_2 0)
      (set `self.maxPage` 1)
      (else
        (set `self.maxPage` _returnvalue_2)))
    (else
      (set `self.maxPage` (+ _returnvalue_2 1))))
  (message `/Game/Blueprints/InventoryManager.SetItemSlot` self))

(event `self.SlotCollision4.OnInputTouchEnd`
  (params (FingerIndex :type "ETouchIndex Enum" :default "Touch1") (TouchedComponent :type "PrimitiveComponent Object Reference"))
  ;[1 1 1] 아이템 슬롯4 클릭 이벤트
  (if (== TouchedComponent (`self.enableButton`))
    (message `/Game/Blueprints/InventoryManager.SelectItem` (`self.attachToScene`) (+ (* (- (`self.nowPage`) 1) 4) 3))
    (`self.CloseInventory`)))

(event `self.SlotCollision4.OnInputTouchBegin`
  (params (FingerIndex :type "ETouchIndex Enum" :default "Touch1") (TouchedComponent :type "PrimitiveComponent Object Reference"))
  ;[1 1 1] 아이템 슬롯4 클릭 이벤트
  (set `self.enableButton` TouchedComponent))

(event `self.PrevPage_Button.OnInputTouchEnd`
  (params (FingerIndex :type "ETouchIndex Enum" :default "Touch1") (TouchedComponent :type "PrimitiveComponent Object Reference"))
  ;[1 1 1] 이전 페이지로
  (if (== (`self.enableButton`) TouchedComponent)
    (if (> (`self.nowPage`) 1)
      (set `self.nowPage` (+ -1 (`self.nowPage`)))
      (message `/Game/Blueprints/InventoryManager.SetItemSlot` self))))

(event `CloseInventory`
  ;[1 1 1] 인벤토리 닫기
  (`self.SetActorHiddenInGame` true)
  (`self.SetActorEnableCollision` false)
  (`self.SetActorEnableCollision` (`self.attachToScene`) true))

(event `self.PrevPage_Button.OnInputTouchBegin`
  (params (FingerIndex :type "ETouchIndex Enum" :default "Touch1") (TouchedComponent :type "PrimitiveComponent Object Reference"))
  ;[1 1 1] 이전 페이지로
  (set `self.enableButton` TouchedComponent))

(event `self.NextPage_Button.OnInputTouchEnd`
  (params (FingerIndex :type "ETouchIndex Enum" :default "Touch1") (TouchedComponent :type "PrimitiveComponent Object Reference"))
  ;[1 1 1] 다음 페이지로
  (if (== (`self.enableButton`) TouchedComponent)
    (if (< (`self.nowPage`) (`self.maxPage`))
      (set `self.nowPage` (+ 1 (`self.nowPage`)))
      (message `/Game/Blueprints/InventoryManager.SetItemSlot` self))))

(event `self.NextPage_Button.OnInputTouchBegin`
  (params (FingerIndex :type "ETouchIndex Enum" :default "Touch1") (TouchedComponent :type "PrimitiveComponent Object Reference"))
  ;[1 1 1] 다음 페이지로
  (set `self.enableButton` TouchedComponent))

(fn `UserConstructionScript`)